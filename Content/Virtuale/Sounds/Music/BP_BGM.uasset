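; Background music Blueprint that plays through an audio component and switches tracks when the police system fires its POLICE event.
; On BeginPlay it applies the music volume stored in the game instance and binds to its music-change event to keep the volume in sync.
; It also binds to every police singleton; that event plays the Little Red Snitches prelude, then swaps to the loop after a short fixed delay.
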(event Custom|SetVolume
  (Audio|Components|Audio|SetVolumeMultiplier (Variables|Default|GetAudio) (Variables|/Game/AdvancedTurnBasedTileToolkit/Maps/MP/Core/BP_GI_ATBTT.BP_GI_ATBTT_C|GetMusicVolume (stale EventBeginPlay _asbp_gi_atbtt)) :!class /Script/Engine.AudioComponent))

(event Custom|CustomEvent
  (bind _audio (Variables|Default|GetAudio))
  (Audio|Components|Audio|SetSound _audio "/Game/Virtuale/Sounds/Music/LiittleRedSnitches-Prelude.LiittleRedSnitches-Prelude")
  (Utilities|FlowControl|Delay 1.7)
  (Audio|Components|Audio|SetSound _audio "/Game/Virtuale/Sounds/Music/LittleRedSnitches-Loop.LittleRedSnitches-Loop"))

(event EventBeginPlay
  (bind _asbp_gi_atbtt (Utilities|Casting|CastToBP_GI_ATBTT (Game|GetGameInstance)))
  (EventDispatchers|BindEventtoMusicChange _asbp_gi_atbtt (delegate Custom|SetVolume))
  (bind _outactors (Actor|GetAllActorsOfClass "/Game/Virtuale/AI/Blueprints/BP_PoliceSystem_Singleton.BP_PoliceSystem_Singleton_C"))
  (for _array_element _outactors
    (EventDispatchers|BindEventtoPOLICE _array_element (delegate Custom|CustomEvent)))
  (Audio|Components|Audio|SetVolumeMultiplier (Variables|Default|GetAudio) (Variables|/Game/AdvancedTurnBasedTileToolkit/Maps/MP/Core/BP_GI_ATBTT.BP_GI_ATBTT_C|GetMusicVolume _asbp_gi_atbtt) :!class /Script/Engine.AudioComponent))

(fn ConstructionScript)