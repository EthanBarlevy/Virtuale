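; Escape node actor that marks a grid cell and links to a parent node to form a chain of escape indexes, apparently for AI.
; The construction script uses the grid manager to convert the actor's location into its stored grid index.
; GetEscapeIndexes recursively appends each node's index up the parent chain and returns the accumulated list.
; The static mesh is destroyed on BeginPlay, so the node has no mesh during play.
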(event EventBeginPlay
  (|CallParentFunction)
  (CallFunction|RemoveMesh))

(event EventTick
  (params (DeltaSeconds :type Float%20%28single-precision%29))
  (|CallParentFunction DeltaSeconds) ; This node is disabled and will not be called.\nDrag off pins to build functionality.
)

(fn ConstructionScript
  (|CallParentFunction)
  (Variables|Default|SetGridIndex (Default|ConvertLocationtoIndex3DNaive (.GridManager (CallFunction|GetGridManager)) (Transformation|GetActorLocation))))

(fn RemoveMesh
  (Components|DestroyComponent (Variables|Default|GetStaticMesh)))

(fn GetEscapeIndexes
  (params (Indexes :type Array%20of%20Integers))
  (Utilities|Array|Add Indexes (Variables|Default|GetGridIndex))
  (if (Utilities|IsValid (Variables|Default|GetParentNode))
    (bind _outdexes (CallFunction|GetEscapeIndexes (Variables|Default|GetParentNode) Indexes))
    (return _outdexes)
    (else
      (return Indexes))))