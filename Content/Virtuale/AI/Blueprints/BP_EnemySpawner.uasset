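; Enemy spawner that places debug AI units on random cells of the grid at level start.
; After a short delay it gets the grid manager and makes SpawnCount attempts, copying stats from the EnemySpawn actor.
; Occupied picks use up an attempt, and each lookup re-rolls the random index, so the checked cell can differ from the spawn cell.
; Spawned units register with the grid manager at index 0.
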(event EventBeginPlay
  (bind (_bvalid _gridmanager) (CallFunction|GetGridManager))
  (Utilities|FlowControl|Delay 0.1)
  (if _bvalid
    (Variables|Default|SetGrid%20Manager%20Ref _gridmanager)
    (Utilities|IsValid (Variables|Default|GetEnemySpawn)
      (:Is%20Valid
        (while (!= (Variables|Default|GetSpawnCount) 0)
          (CallFunction|RandomSpawnLocation))))))

(event Collision|EventActorBeginOverlap
  (params (OtherActor :type Actor%20Object%20Reference)))

(event EventTick
  (params (DeltaSeconds :type Float%20%28single-precision%29)))

(fn ConstructionScript)

(fn SpawnEnemy
  (params (SpawnLocation :type Vector))
  (bind _enemyspawn (Variables|Default|GetEnemySpawn))
  (bind _returnvalue (Game|SpawnActorfromClass "/Game/Virtuale/AI/Blueprints/BP_Unit_AI_Debug.BP_Unit_AI_Debug_C" (Math|Transform|MakeTransform SpawnLocation (Transformation|GetActorRotation _enemyspawn) "1.000000,1.000000,1.000000") (Variables|/Script/Engine.Actor|GetSpawnCollisionHandlingMethod _enemyspawn) "MultiplyWithRoot" (Components|GetOwner _enemyspawn) (Variables|/Game/AdvancedTurnBasedTileToolkit/Core/Units/BP_Unit.BP_Unit_C|GetMaxAP _enemyspawn) (Variables|/Game/AdvancedTurnBasedTileToolkit/Core/Units/BP_Unit.BP_Unit_C|GetCurrentAP _enemyspawn) (Variables|/Game/AdvancedTurnBasedTileToolkit/Core/Units/BP_Unit.BP_Unit_C|GetMove _enemyspawn) (Variables|/Game/AdvancedTurnBasedTileToolkit/Core/Units/BP_Unit.BP_Unit_C|GetRange _enemyspawn) (Variables|/Game/AdvancedTurnBasedTileToolkit/Core/Units/BP_Unit.BP_Unit_C|GetMinimumRange _enemyspawn) (Variables|/Game/AdvancedTurnBasedTileToolkit/Core/Units/BP_Unit.BP_Unit_C|GetMaxHealth _enemyspawn) (Variables|/Game/AdvancedTurnBasedTileToolkit/Core/Units/BP_Unit.BP_Unit_C|GetCurrentHealth _enemyspawn) (Variables|/Game/AdvancedTurnBasedTileToolkit/Core/Units/BP_Unit.BP_Unit_C|GetDamage _enemyspawn) (Variables|/Game/AdvancedTurnBasedTileToolkit/Core/Units/BP_Unit.BP_Unit_C|GetInitiative _enemyspawn) true "NewEnumerator1" true "/Game/AdvancedTurnBasedTileToolkit/Units/Puppets/BP_Actor_Puppet_Debug.BP_Actor_Puppet_Debug_C" (Variables|/Script/Engine.Actor|GetInstigator _enemyspawn)))
  (Utilities|IsValid _returnvalue
    (:Is%20Valid
      (Default|AddUnittoGrid (Variables|Default|GetGrid%20Manager%20Ref) _returnvalue))))

(fn RandomSpawnLocation
  (bind _grid_manager_ref (Variables|Default|GetGrid%20Manager%20Ref))
  (bind _gridlocations (Variables|/Game/AdvancedTurnBasedTileToolkit/Core/Grid/BP_GridManager.BP_GridManager_C|GetGridLocations _grid_manager_ref))
  (Variables|Default|SetSpawnCount (- (Variables|Default|GetSpawnCount) 1))
  (bind _keys (Utilities|Map|Keys _gridlocations))
  (if (not (Utilities|Map|Contains (Variables|/Game/AdvancedTurnBasedTileToolkit/Core/Grid/BP_GridManager.BP_GridManager_C|GetGridUnits (Variables|Default|GetGrid%20Manager%20Ref)) (Utilities|Array|Get(acopy) _keys (Math|Random|RandomIntegerinRange 1 (- (Utilities|Map|Length _gridlocations) 1)))))
    (if (.ReturnValue (Utilities|Map|Find _gridlocations (Utilities|Array|Get(acopy) _keys (Math|Random|RandomIntegerinRange 1 (- (Utilities|Map|Length _gridlocations) 1)))))
      (CallFunction|SpawnEnemy (.Value (Utilities|Map|Find _gridlocations (Utilities|Array|Get(acopy) _keys (Math|Random|RandomIntegerinRange 1 (- (Utilities|Map|Length _gridlocations) 1)))))))))