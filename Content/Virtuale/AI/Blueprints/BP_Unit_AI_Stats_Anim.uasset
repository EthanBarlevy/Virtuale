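; Grid-based AI unit Blueprint that adds player proximity checks and status affects to its parent unit class.
; IsPlayerInRange finds the closest Player-tagged actor by diamond-shaped tile distance via the grid manager, and the unit select display is only queued within 15 tiles.
; Unconscious, swoon and distraction setters save the previous state and set the affect, with distraction also storing a search location.
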(event EventBeginPlay
  (|CallParentFunction)
  (Variables|Default|SetState (Variables|Default|GetState)))

(event Collision|EventActorBeginOverlap
  (params (OtherActor :type Actor%20Object%20Reference)))

(event EventTick
  (params (DeltaSeconds :type Float%20%28single-precision%29)))

(event EventSpawnPuppet
  (|CallParentFunction))

(event EventQueueShowUnitSelect
  (bind _playerinrange (CallFunction|IsPlayerinRange 15))
  (if _playerinrange
    (|CallParentFunction)))

(fn ConstructionScript
  (|CallParentFunction))

(fn IsPlayerinRange
  (params (PlayerRange :type Integer))
  (bind _gridmanagerref (Variables|Default|GetGridManagerRef))
  (bind _gridmanagerref_2 (Variables|Default|GetGridManagerRef))
  (bind _outactors (Actor|GetAllActorswithTag "Player"))
  (for _array_element _outactors
    (if (Utilities|IsValid (LocalVariables|GetClosestPlayer))
      (if (< (Default|FindDistanceIinTilesBetweenIndexes _gridmanagerref (Variables|Default|GetGridIndex) (Default|ConvertLocationtoIndex3DNaive _gridmanagerref (Transformation|GetActorLocation _array_element)) true) (LocalVariables|GetDistance))
        (LocalVariables|SetClosestPlayer _array_element)
        (LocalVariables|SetDistance (Default|FindDistanceIinTilesBetweenIndexes _gridmanagerref (Variables|Default|GetGridIndex) (Default|ConvertLocationtoIndex3DNaive _gridmanagerref (Transformation|GetActorLocation _array_element)) true)))
      (else
        (bind _output_get (LocalVariables|SetClosestPlayer _array_element))
        (LocalVariables|SetDistance (Default|FindDistanceIinTilesBetweenIndexes _gridmanagerref_2 (Variables|Default|GetGridIndex) (Default|ConvertLocationtoIndex3DNaive _gridmanagerref_2 (Transformation|GetActorLocation _output_get)) true)))))
  (return (< (LocalVariables|GetDistance) PlayerRange) (LocalVariables|GetDistance)))

(fn SetUnconsciousAffect
  (Variables|Default|SetPrevState (Variables|Default|GetState))
  (Variables|Default|SetAffects "NewEnumerator1"))

(fn SetSwoonAffect
  (Variables|Default|SetPrevState (Variables|Default|GetState))
  (Variables|Default|SetAffects "NewEnumerator3"))

(fn SetDistractionAffectLocation
  (params (Index :type Integer))
  (Variables|Default|SetCurrentSearchLocation (Default|ConvertIndextoLocation (.GridManager (CallFunction|GetGridManager)) Index 0.0))
  (Variables|Default|SetPrevState (Variables|Default|GetState))
  (Variables|Default|SetAffects "NewEnumerator2"))

(fn SetDistractionAffectIndex
  (params (Location :type Vector))
  (Variables|Default|SetPrevState (Variables|Default|GetState))
  (Variables|Default|SetCurrentSearchLocation Location)
  (Variables|Default|SetAffects "NewEnumerator2")
  (Variables|Default|SetAffectsDelayTurns 3))