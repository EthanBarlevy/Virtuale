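; BP_GuardPuppet is a guard character puppet with toggleable hat and weapon props.
; AddHat flips a hat flag, then sets or clears the AdditionalProp mesh.
; WeaponSwap flips HasWeapon and assigns the scoped pistol mesh to Weapon, both for the Pistol type when on and unconditionally when off.
; BeginPlay is empty, the construction script only calls its parent, and a ShowOnlyActorComponents call is unwired.
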(event EventBeginPlay)

(fn ConstructionScript
  (|CallParentFunction))

(fn AddHat
  (bind _additionalprop (Variables|Default|GetAdditionalProp))
  (bind _output_get (Variables|Default|Sethat (not (Variables|Default|Gethat))))
  (if _output_get
    (Components|StaticMesh|SetStaticMesh _additionalprop "/Game/Virtuale/Models/hat.hat")
    (else
      (Components|StaticMesh|SetStaticMesh _additionalprop 0))))

(fn WeaponSwap
  (params (WeaponType :type E_WeaponType%20Enum :default "NewEnumerator7"))
  (bind _output_get (Variables|Default|SethasWeapon (not (Variables|Default|GethasWeapon))))
  (if _output_get
    (switch Utilities|FlowControl|Switch|SwitchonE_WeaponType WeaponType
      (:NewEnumerator0
        (Components|StaticMesh|SetStaticMesh (Variables|Default|GetWeapon) "/Game/Virtuale/Models/scoped-pistol.scoped-pistol")))
    (else
      (Components|StaticMesh|SetStaticMesh (Variables|Default|GetWeapon) "/Game/Virtuale/Models/scoped-pistol.scoped-pistol"))))