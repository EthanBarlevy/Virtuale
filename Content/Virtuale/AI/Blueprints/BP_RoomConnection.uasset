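; BP_RoomConnection is a placed grid marker that records the tiles of a room and its links to other rooms for AI use.
; Construction stores its grid index; BeginPlay destroys its mesh and, after a short delay, fills RoomTiles with every tile reached by range-limited GridManager pathfinding from that index.
; IsUnitInNearByRoom searches the connected rooms' tiles for a unit's index and returns that connection's exit index.
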(event EventBeginPlay
  (|CallParentFunction)
  (CallFunction|RemoveMesh)
  (Utilities|FlowControl|Delay 2.0)
  (CallFunction|GetAllTilesinRoom))

(event EventTick
  (params (DeltaSeconds :type Float%20%28single-precision%29))
  (|CallParentFunction DeltaSeconds) ; This node is disabled and will not be called.\nDrag off pins to build functionality.
)

(fn ConstructionScript
  (|CallParentFunction)
  (Variables|Default|SetGridIndex (Default|ConvertLocationtoIndex3DNaive (.GridManager (CallFunction|GetGridManager)) (Transformation|GetActorLocation))))

(fn RemoveMesh
  (Components|DestroyComponent (Variables|Default|GetStaticMesh)))

(fn GetAllTilesinRoom
  (bind _output_get (Variables|Default|SetGrid%20Manager%20Ref (.GridManager (CallFunction|GetGridManager))))
  (bind _pathsmap (Default|RunPathfinding _output_get (Variables|Default|GetGridIndex) 30 "/Game/AdvancedTurnBasedTileToolkit/Core/Pathfinding/BP_Path.BP_Path_C"))
  (bind _keys (Utilities|Map|Keys _pathsmap))
  (Variables|Default|SetRoomTiles _keys))

(fn IsUnitinNearbyRoom
  (params (UnitIndex :type Integer))
  (bind _keys (Utilities|Map|Keys (Variables|Default|GetConnections)))
  (bind _array_element (Utilities|Array|ForEachLoopwithBreak _keys)
    (:LoopBody
      (if (Utilities|Array|ContainsItem (Variables|BP_RoomConnection_C|GetRoomTiles _array_element) UnitIndex)
        (return true (.Value (Utilities|Map|Find (Variables|Default|GetConnections) _array_element)))))
    (:Completed
      (return false 0))))