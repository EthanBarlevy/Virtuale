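; Area spawner that places a set number of AI enemy units on random grid cells around itself at game start.
; On BeginPlay it removes its mesh, waits briefly, then asks the grid manager for cells in range, optionally diamond-shaped.
; Each spawn creates a debug AI unit at a random cell, copies stats from the EnemySpawn reference and registers it with the grid.
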(event EventBeginPlay
  (bind (_bvalid _gridmanager) (CallFunction|GetGridManager))
  (|CallParentFunction)
  (CallFunction|RemoveMesh)
  (Utilities|FlowControl|Delay 0.1)
  (if _bvalid
    (Variables|Default|SetGrid%20Manager%20Ref _gridmanager)
    (Utilities|IsValid (Variables|Default|GetEnemySpawn)
      (:Is%20Valid
        (bind _inrangetiles (Default|GetIndexesinRange (Variables|Default|GetGrid%20Manager%20Ref) (Default|ConvertLocationtoIndex3DNaive (Variables|Default|GetGrid%20Manager%20Ref) (Transformation|GetActorLocation)) (Variables|Default|GetArea) (Variables|Default|GetDiamondShape) false))
        (while (!= (Variables|Default|GetSpawnAmount) 0)
          (CallFunction|RandomSpawn _inrangetiles)
          (Variables|Default|SetSpawnAmount (- (Variables|Default|GetSpawnAmount) 1)))))))

(event Collision|EventActorBeginOverlap
  (params (OtherActor :type Actor%20Object%20Reference))
  (|CallParentFunction OtherActor) ; This node is disabled and will not be called.\nDrag off pins to build functionality.
)

(event EventTick
  (params (DeltaSeconds :type Float%20%28single-precision%29))
  (|CallParentFunction DeltaSeconds) ; This node is disabled and will not be called.\nDrag off pins to build functionality.
)

(fn ConstructionScript
  (|CallParentFunction))

(fn SpawnEnemy
  (params (SpawnPoint :type Vector))
  (bind _enemyspawn (Variables|Default|GetEnemySpawn))
  (bind _returnvalue (Game|SpawnActorfromClass "/Game/Virtuale/AI/Blueprints/BP_Unit_AI_Debug.BP_Unit_AI_Debug_C" (Math|Transform|MakeTransform SpawnPoint (Transformation|GetActorRotation _enemyspawn) "1.000000,1.000000,1.000000") (Variables|/Script/Engine.Actor|GetSpawnCollisionHandlingMethod _enemyspawn) "MultiplyWithRoot" (Components|GetOwner _enemyspawn) (Variables|/Game/AdvancedTurnBasedTileToolkit/Core/Units/BP_Unit.BP_Unit_C|GetMaxAP _enemyspawn) (Variables|/Game/AdvancedTurnBasedTileToolkit/Core/Units/BP_Unit.BP_Unit_C|GetCurrentAP _enemyspawn) (Variables|/Game/AdvancedTurnBasedTileToolkit/Core/Units/BP_Unit.BP_Unit_C|GetMove _enemyspawn) (Variables|/Game/AdvancedTurnBasedTileToolkit/Core/Units/BP_Unit.BP_Unit_C|GetRange _enemyspawn) (Variables|/Game/AdvancedTurnBasedTileToolkit/Core/Units/BP_Unit.BP_Unit_C|GetMinimumRange _enemyspawn) (Variables|/Game/AdvancedTurnBasedTileToolkit/Core/Units/BP_Unit.BP_Unit_C|GetMaxHealth _enemyspawn) (Variables|/Game/AdvancedTurnBasedTileToolkit/Core/Units/BP_Unit.BP_Unit_C|GetCurrentHealth _enemyspawn) (Variables|/Game/AdvancedTurnBasedTileToolkit/Core/Units/BP_Unit.BP_Unit_C|GetDamage _enemyspawn) (Variables|/Game/AdvancedTurnBasedTileToolkit/Core/Units/BP_Unit.BP_Unit_C|GetInitiative _enemyspawn) true "NewEnumerator1" true "/Game/AdvancedTurnBasedTileToolkit/Units/Puppets/BP_Actor_Puppet_Debug.BP_Actor_Puppet_Debug_C" (Variables|/Script/Engine.Actor|GetInstigator _enemyspawn)))
  (Utilities|IsValid _returnvalue
    (:Is%20Valid
      (Default|AddUnittoGrid (Variables|Default|GetGrid%20Manager%20Ref) _returnvalue))))

(fn RemoveMesh
  (Components|DestroyComponent (Variables|Default|GetStaticMesh)))

(fn RandomSpawn
  (params (Indexes :type Array%20of%20Integers))
  (bind _returnvalue (Utilities|Array|Length Indexes))
  (bind _returnvalue_2 (- _returnvalue 1))
  (bind _returnvalue_3 (Math|Random|RandomIntegerinRange 0 _returnvalue_2))
  (bind _output (Utilities|Array|Get(acopy) Indexes _returnvalue_3))
  (Utilities|Array|RemoveIndex Indexes _output)
  (CallFunction|SpawnEnemy (Default|ConvertIndextoLocation (Variables|Default|GetGrid%20Manager%20Ref) _output 0.0)))