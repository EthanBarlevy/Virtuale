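; Singleton police alarm system that runs a turn-based countdown and spawns guard reinforcements while it is active.
; The construction script destroys any other instances to keep one per level.
; StartCountDown calls the police and sets the initial count by whether a single "Vlad"-tagged actor exists.
; DoTurn decrements the count, which triggers nothing at zero, and spawns capped batches of guards at random "GuardSpawn" spawner areas.
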(event EventBeginPlay)

(event Collision|EventActorBeginOverlap
  (params (OtherActor :type Actor%20Object%20Reference)))

(event EventTick
  (params (DeltaSeconds :type Float%20%28single-precision%29)))

(fn ConstructionScript
  (bind _outactors (Actor|GetAllActorsOfClass "BP_PoliceSystem_Singleton_C"))
  (if (> (Utilities|Array|Length _outactors) 1)
    (for _array_element _outactors
      (if (!= _array_element self)
        (Actor|DestroyActor _array_element)))))

(fn CountDownTimer
  (if (Variables|Default|GetTimerActive)
    (bind _result (Math|Integer|DecrementInt (Variables|Default|GetPoliceCountDown))
      (:%20%20
        (if (<= _result 0)
          _)))))

(fn StartCountDown
  (Variables|Default|SetTimerActive true)
  (Default|CallPOLICE)
  (bind _outactors (Actor|GetAllActorswithTag "Vlad"))
  (if (== (Utilities|Array|Length _outactors) 1)
    (if (== (Variables|Default|GetPoliceCountDown) 69420)
      (Variables|Default|SetPoliceCountDown (Variables|Default|GetCountDownStart)))
    (elif (== (Variables|Default|GetPoliceCountDown) 69420)
      (Variables|Default|SetPoliceCountDown (Variables|Default|GetValdlessTimer)))))

(fn IsCountDownActive
  (return (Variables|Default|GetTimerActive)))

(fn DoTurn
  (bind _guardspawneractor (LocalVariables|GetGuardSpawnerActor))
  (bind _guardspawneractor_2 (LocalVariables|GetGuardSpawnerActor))
  (bind _returnvalue (Utilities|Array|Length _guardspawneractor_2))
  (bind _returnvalue_2 (- _returnvalue 1))
  (bind _returnvalue_3 (Math|Random|RandomIntegerinRange 0 _returnvalue_2))
  (bind _output (Utilities|Array|Get(acopy) _guardspawneractor _returnvalue_3))
  (if (Variables|Default|GetTimerActive)
    (CallFunction|CountDownTimer)
    (bind _outactors (Actor|GetAllActorswithTag "Guard"))
    (LocalVariables|SetSpawnGuardAmount (- 25 (Utilities|Array|Length _outactors)))
    (if (not (> (Utilities|Array|Length _outactors) 25))
      (bind _outactors_2 (Actor|GetAllActorswithTag "GuardSpawn"))
      (for _array_element _outactors_2
        (bind _asbp_enemy_spawner_area (Utilities|Casting|CastToBP_EnemySpawnerArea _array_element))
        (Utilities|Array|Add (LocalVariables|GetGuardSpawnerActor) _asbp_enemy_spawner_area))
      (if (!= _returnvalue 0)
        (for _index (range 0 (select (< (LocalVariables|GetSpawnGuardAmount) (LocalVariables|GetGuardSpawnLimit)) (LocalVariables|GetSpawnGuardAmount) (LocalVariables|GetGuardSpawnLimit)))
          (bind _indexes (Default|GetSpawnArea _output))
          (Default|RandomSpawn _output _indexes))
        (else
          (Development|PrintString "No Spawners with Tag \"GuardSpawn\" in the level" true true "(R=0.000000,G=0.660000,B=1.000000,A=1.000000)" 5.0))))))