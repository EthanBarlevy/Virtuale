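; BP_PatrolLocations holds a list of patrol locations and a current index for stepping through an AI patrol route.
; GetCurrentLocation reads the entry at the index, while GetNextLocation increments it and wraps to the first entry at the end.
; GetPreviousLocation decrements it but reuses the upper-bound check, so it resets to the last entry at the array's end rather than wrapping below zero.
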(fn GetNextLocation
  (bind _patrollocations (Variables|Default|GetPatrolLocations))
  (if (< (+ 1 (Variables|Default|GetCurrentIndex)) (Utilities|Array|Length (Variables|Default|GetPatrolLocations)))
    (bind _result (Math|Integer|IncrementInt (Variables|Default|GetCurrentIndex))
      (:%20%20
        (return (Utilities|Array|Get(acopy) _patrollocations _result))))
    (else
      (bind _output_get (Variables|Default|SetCurrentIndex 0))
      (return (Utilities|Array|Get(acopy) _patrollocations _output_get)))))

(fn GetCurrentLocation
  (return (Utilities|Array|Get(acopy) (Variables|Default|GetPatrolLocations) (Variables|Default|GetCurrentIndex))))

(fn GetPreviousLocation
  (bind _patrollocations (Variables|Default|GetPatrolLocations))
  (bind _patrollocations_2 (Variables|Default|GetPatrolLocations))
  (bind _returnvalue (Utilities|Array|Length _patrollocations))
  (if (< (+ 1 (Variables|Default|GetCurrentIndex)) _returnvalue)
    (bind _result (Math|Integer|DecrementInt (Variables|Default|GetCurrentIndex))
      (:%20%20
        (return (Utilities|Array|Get(acopy) _patrollocations_2 _result))))
    (else
      (bind _output_get (Variables|Default|SetCurrentIndex (- _returnvalue 1)))
      (return (Utilities|Array|Get(acopy) _patrollocations_2 _output_get)))))