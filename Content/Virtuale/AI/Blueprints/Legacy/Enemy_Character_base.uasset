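; Legacy base enemy character Blueprint that supplies patrol data and movement speed control for AI.
; When patrol points exist, the construction script writes the first point and the random-patrol flag to the controller's Blackboard.
; NextPatrolLocation steps an index through the point array, wrapping to the start, and returns that location.
; UpdateWalkSpeed sets the character movement's maximum walk speed.
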(fn ConstructionScript
  (bind _returnvalue (Pawn|GetController))
  (bind _returnvalue_2 (AI|GetBlackboard _returnvalue))
  (if (> (Utilities|Array|Length (Variables|Default|GetPL)) 0)
    (AI|Components|Blackboard|SetValueasVector _returnvalue_2 (LocalVariables|GetPatrolLocation) (Utilities|Array|Get(acopy) (Variables|Default|GetPL)))
    (AI|Components|Blackboard|SetValueasBool _returnvalue_2 (Variables|Default|GetUseRandomPatrol) (Variables|Default|GetRandomPatrol))))

(fn UpdateWalkSpeed
  (params (New%20Speed :type Float%20%28double-precision%29))
  (Variables|/Script/Engine.CharacterMovementComponent|SetMaxWalkSpeed (Variables|Character|GetCharacterMovement) New%20Speed))

(fn NextPatrolLocation
  (bind _pl (Variables|Default|GetPL))
  (bind _returnvalue (Utilities|Array|Length _pl))
  (if (> _returnvalue 0)
    (if (< (+ 1 (Variables|Default|GetPatrolIndex)) _returnvalue)
      (bind _result (Math|Integer|IncrementInt (Variables|Default|GetPatrolIndex))
        (:%20%20
          (return (Utilities|Array|Get(acopy) (Variables|Default|GetPL) _result))))
      (else
        (bind _output_get (Variables|Default|SetPatrolIndex 0))
        (return (Utilities|Array|Get(acopy) (Variables|Default|GetPL) _output_get))))))