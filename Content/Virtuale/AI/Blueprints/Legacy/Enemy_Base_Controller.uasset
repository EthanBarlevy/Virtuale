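; Base enemy AI controller that runs BT_Enemy_Base and drives its GuardState blackboard enum between patrol, search, chase and engage.
; Sensing a Player-tagged actor cancels pending timers, stores the target and switches to chase unless already chasing or engaging.
; Other perception updates start a line-of-sight timer that records the target's current location, clears it and switches to search.
; ChangeStateAfterTime schedules StateChange by name; the search-to-patrol timer call is unwired.
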(event OnTargetPerceptionUpdated(AIPerception)
  (params (Actor :type Actor%20Object%20Reference) (Stimulus :type AI%20Stimulus%20Structure))
  (bind _blackboard (Variables|Default|GetBlackboard))
  (bind _blackboard_2 (Variables|Default|GetBlackboard))
  (bind _guardstate (Variables|Default|GetGuardState))
  (bind _returnvalue (Class|BlackboardComponent|GetValueasEnum _blackboard_2 _guardstate))
  (if (and (Actor|ActorHasTag Actor "Player") (.bSuccessfullySensed (Utilities|Struct|BreakAIStimulus Stimulus)))
    ;[0.3531 0.3531 0.3531] Change to chase state
    (Utilities|Time|ClearandInvalidateTimerbyHandle (Variables|Default|GetEnemyTimer))
    (Utilities|Time|ClearandInvalidateTimerbyHandle (Variables|Default|GetSearchEvent))
    (AI|Components|Blackboard|SetValueasBool _blackboard (Variables|Default|GetHasLineOfSight) true)
    (AI|Components|Blackboard|SetValueasObject _blackboard (Variables|Default|GetEnemyActor) Actor)
    (if (and (!= _returnvalue 2) (!= _returnvalue 3))
      (AI|Components|Blackboard|SetValueasEnum _blackboard_2 _guardstate 2)
      (Development|PrintString "Chasing Player"))
    (else
      ;[0.3281 0.3281 0.3281] Set state to search the last known place
      (bind _returnvalue_2 (Utilities|Time|SetTimerbyEvent (delegate Custom|StartEnemyTimer) (Variables|Default|GetLine%20Of%20Sight%20Timer)))
      (Variables|Default|SetEnemyTimer _returnvalue_2))))

(event Custom|StartEnemyTimer
  (bind _blackboard (Variables|Default|GetBlackboard))
  ;[0.3281 0.3281 0.3281] Set state to search the last known place
  (Development|PrintString "Searching for Player")
  (AI|Components|Blackboard|SetValueasBool _blackboard (Variables|Default|GetHasLineOfSight) false)
  (bind _asactor (Utilities|Casting|CastToActor (AI|Components|Blackboard|GetValueasObject _blackboard (Variables|Default|GetEnemyActor))))
  (AI|Components|Blackboard|SetValueasVector _blackboard (Variables|Default|GetInitailSearchLocation) (Transformation|GetActorLocation _asactor))
  (AI|Components|Blackboard|SetValueasObject _blackboard (Variables|Default|GetEnemyActor) 0)
  (AI|Components|Blackboard|SetValueasEnum _blackboard (Variables|Default|GetGuardState) 1))

(event Custom|StartSearchTimer
  ;[0.1698 0.1698 0.1698] Searching to Patrol
  (AI|Components|Blackboard|SetValueasEnum (Variables|Default|GetBlackboard) (Variables|Default|GetGuardState))
  (Development|PrintString "Hello"))

(event EventPossess
  (params (PossessedPawn :type Pawn%20Object%20Reference))
  (AI|RunBehaviorTree "/Game/Virtuale/AI/Blueprints/Legacy/BT_Enemy_Base.BT_Enemy_Base"))

(fn ConstructionScript)

(fn ChangeStateAfterTime
  (params (Time :type Float%20%28double-precision%29) (New%20State :type EGuardState%20Enum :default "NewEnumerator0"))
  (if (not (Utilities|Time|IsTimerActivebyHandle (Variables|Default|GetSearchEvent)))
    (Variables|Default|SetNewState New%20State)
    (bind _returnvalue (Utilities|Time|SetTimerbyFunctionName 0 "StateChange" Time))
    (Variables|Default|SetSearchEvent _returnvalue)))

(fn StateChange
  (params (NewState :type EGuardState%20Enum :default "NewEnumerator0"))
  (AI|Components|Blackboard|SetValueasEnum (Variables|Default|GetBlackboard) (Variables|Default|GetGuardState) NewState)
  (Development|PrintString "State is being Changed"))