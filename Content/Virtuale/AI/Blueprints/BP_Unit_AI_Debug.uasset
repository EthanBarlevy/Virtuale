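; BP_Unit_AI_Debug is an AI unit Blueprint for grid-based, turn-based play that adds unconscious, swoon and distraction affects.
; Each affect setter saves the current state; distraction also sets a search location from a vector or grid index, with only the vector version setting a turn delay.
; Unit selection is queued only when the unit is alerted or a grid move-range search finds an allied-faction unit.
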(event EventBeginPlay
  (|CallParentFunction)
  (Variables|States|SetPrevState (Variables|States|GetState)))

(event Collision|EventActorBeginOverlap
  (params (OtherActor :type Actor%20Object%20Reference)))

(event EventTick
  (params (DeltaSeconds :type Float%20%28single-precision%29)))

(event EventQueueShowUnitSelect
  (bind _inrange (CallFunction|InPlayerRange))
  (if _inrange
    (|CallParentFunction)))

(fn ConstructionScript
  (|CallParentFunction))

(fn SetUnconsciousAffect
  (Variables|States|SetPrevState (Variables|States|GetState))
  (Variables|Affects|SetAffects "NewEnumerator1"))

(fn SetSwoonAffect
  (Variables|States|SetPrevState (Variables|States|GetState))
  (Variables|Affects|SetAffects "NewEnumerator3"))

(fn SetDistractionAffectLocation
  (params (Location :type Vector))
  (Variables|States|SetPrevState (Variables|States|GetState))
  (Variables|States|SetCurrentSearchLocation Location)
  (Variables|Affects|SetAffects "NewEnumerator2")
  (Variables|Affects|SetAffectsDelayTurns 3))

(fn SetDistractionAffectGridIndex
  (params (Index :type Integer))
  (Variables|States|SetCurrentSearchLocation (Default|ConvertIndextoLocation (.GridManager (CallFunction|GetGridManager)) Index 0.0))
  (Variables|States|SetPrevState (Variables|States|GetState))
  (Variables|Affects|SetAffects "NewEnumerator2"))

(fn InPlayerRange
  (bind _btargetfound (Default|FindClosestUnitinMoveRange (Variables|Default|GetGridManagerRef) (Variables|Default|GetGridIndex) 15 (Variables|Default|GetPathfindingType) (Variables|Default|GetAlliedFactions) true true))
  (return (or _btargetfound (Variables|Default|GetIsAlearted))))