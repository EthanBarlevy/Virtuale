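; Level marker for a grid-based tactics game that spawns an AI-controlled enemy unit.
; RandomSpawnLocation gets grid indexes within Area, optionally diamond-shaped, but uses only their count, converting a random integer below it directly into a location.
; SpawnEnemy creates a debug AI unit there with stats copied from the EnemySpawn reference, then registers it with the grid manager at index zero.
; RemoveMesh destroys the marker's mesh; nothing here calls it or RandomSpawnLocation.
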(event EventBeginPlay
  (|CallParentFunction))

(event Collision|EventActorBeginOverlap
  (params (OtherActor :type Actor%20Object%20Reference))
  (|CallParentFunction OtherActor) ; This node is disabled and will not be called.\nDrag off pins to build functionality.
)

(event EventTick
  (params (DeltaSeconds :type Float%20%28single-precision%29))
  (|CallParentFunction DeltaSeconds) ; This node is disabled and will not be called.\nDrag off pins to build functionality.
)

(fn ConstructionScript
  (|CallParentFunction))

(fn RandomSpawnLocation
  (bind _grid_manager_ref (Variables|Default|GetGrid%20Manager%20Ref))
  (bind _inrangetiles (Default|GetIndexesinRange _grid_manager_ref (Default|ConvertLocationtoIndex3DNaive _grid_manager_ref (Transformation|GetActorLocation)) (Variables|Default|GetArea) (Variables|Default|GetDiamondShape) false))
  (CallFunction|SpawnEnemy (Default|ConvertIndextoLocation (Variables|Default|GetGrid%20Manager%20Ref) (Math|Random|RandomIntegerinRange 0 (- (Utilities|Array|Length _inrangetiles) 1)) 0.0)))

(fn SpawnEnemy
  (params (SpawnPoint :type Vector))
  (bind _enemyspawn (Variables|Default|GetEnemySpawn))
  (bind _returnvalue (Game|SpawnActorfromClass "/Game/Virtuale/AI/Blueprints/BP_Unit_AI_Debug.BP_Unit_AI_Debug_C" (Math|Transform|MakeTransform SpawnPoint (Transformation|GetActorRotation _enemyspawn) "1.000000,1.000000,1.000000") (Variables|/Script/Engine.Actor|GetSpawnCollisionHandlingMethod _enemyspawn) "MultiplyWithRoot" (Components|GetOwner _enemyspawn) (Variables|/Game/AdvancedTurnBasedTileToolkit/Core/Units/BP_Unit.BP_Unit_C|GetMaxAP _enemyspawn) (Variables|/Game/AdvancedTurnBasedTileToolkit/Core/Units/BP_Unit.BP_Unit_C|GetCurrentAP _enemyspawn) (Variables|/Game/AdvancedTurnBasedTileToolkit/Core/Units/BP_Unit.BP_Unit_C|GetMove _enemyspawn) (Variables|/Game/AdvancedTurnBasedTileToolkit/Core/Units/BP_Unit.BP_Unit_C|GetRange _enemyspawn) (Variables|/Game/AdvancedTurnBasedTileToolkit/Core/Units/BP_Unit.BP_Unit_C|GetMinimumRange _enemyspawn) (Variables|/Game/AdvancedTurnBasedTileToolkit/Core/Units/BP_Unit.BP_Unit_C|GetMaxHealth _enemyspawn) (Variables|/Game/AdvancedTurnBasedTileToolkit/Core/Units/BP_Unit.BP_Unit_C|GetCurrentHealth _enemyspawn) (Variables|/Game/AdvancedTurnBasedTileToolkit/Core/Units/BP_Unit.BP_Unit_C|GetDamage _enemyspawn) (Variables|/Game/AdvancedTurnBasedTileToolkit/Core/Units/BP_Unit.BP_Unit_C|GetInitiative _enemyspawn) true "NewEnumerator1" true "/Game/AdvancedTurnBasedTileToolkit/Units/Puppets/BP_Actor_Puppet_Debug.BP_Actor_Puppet_Debug_C" (Variables|/Script/Engine.Actor|GetInstigator _enemyspawn)))
  (Utilities|IsValid _returnvalue
    (:Is%20Valid
      (Default|AddUnittoGrid (Variables|Default|GetGrid%20Manager%20Ref) _returnvalue))))

(fn RemoveMesh
  (Components|DestroyComponent (Variables|Default|GetStaticMesh)))