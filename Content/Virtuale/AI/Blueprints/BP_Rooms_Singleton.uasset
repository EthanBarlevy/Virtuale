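; BP_Rooms_Singleton is a singleton actor that serves as a lookup for which room a unit occupies.
; On BeginPlay it caches every BP_RoomConnection actor in the level.
; FindUnitRoom searches that cache for the first room whose RoomTiles contain the given UnitIndex, returning a found flag and the room.
; The construction script enforces uniqueness by destroying all other instances; the Find function is empty.
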(event EventBeginPlay
  (bind _outactors (Actor|GetAllActorsOfClass "/Game/Virtuale/AI/Blueprints/BP_RoomConnection.BP_RoomConnection_C"))
  (Variables|Default|SetRoomConnections _outactors))

(fn ConstructionScript
  (bind _outactors (Actor|GetAllActorsOfClass "BP_Rooms_Singleton_C"))
  (if (> (Utilities|Array|Length _outactors) 1)
    (for _array_element _outactors
      (if (!= _array_element self)
        (Actor|DestroyActor _array_element)))))

(fn FindUnitRoom
  (params (Unit%20Index :type Integer))
  (bind _array_element (Utilities|Array|ForEachLoopwithBreak (Variables|Default|GetRoomConnections) :!label _label)
    (:LoopBody
      (if (Utilities|Array|ContainsItem (Variables|/Game/Virtuale/AI/Blueprints/BP_RoomConnection.BP_RoomConnection_C|GetRoomTiles _array_element) Unit%20Index)
        (LocalVariables|SetRoomSpotted _array_element)
        (goto _label Break)))
    (:Completed
      (if (Utilities|IsValid (LocalVariables|GetRoomSpotted))
        (return (Utilities|IsValid (LocalVariables|GetRoomSpotted)) (LocalVariables|GetRoomSpotted))
        (else
          (return (Utilities|IsValid (LocalVariables|GetRoomSpotted)) 0))))))

(fn Find)