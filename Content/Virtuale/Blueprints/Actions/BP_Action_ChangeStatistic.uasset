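; BP_Action_ChangeStatistic is an action that adjusts a chosen stat on its target by a set amount.
; On play, it reads the stat through a GetStatValueMessage call, then writes the current value plus AdjustAmount back through SetStatToValueMessage.
; The action ends with the result of that write, or with true when the target lacks the stat.
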(event EventPlayAction
  (bind (_bhasstat _value) (Class|BPIStats|GetStatValue(Message) (Variables|Default|GetTarget) (Variables|Default|GetStat)))
  (if _bhasstat
    (bind _bsuccess (Class|BPIStats|SetStattoValue(Message) (Variables|Default|GetTarget) (Variables|Default|GetStat) (+ _value (Variables|Default|GetAdjustAmount))))
    (CallFunction|EndAction _bsuccess)
    (else
      (CallFunction|EndAction true))))

(fn ConstructionScript
  (|CallParentFunction))

(fn NewFunction)