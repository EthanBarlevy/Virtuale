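; BP_Action_GiveItem is an action Blueprint that gives an item to a receiving player.
; On PlayAction it looks up the Inventory component on RecevingPlayer and, if valid, adds Object directly to that component's Items.
; It then calls EndAction with true on success, or false when no valid Inventory is found.
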(event EventBeginPlay
  (|CallParentFunction) ; This node is disabled and will not be called.\nDrag off pins to build functionality.
)

(event Collision|EventActorBeginOverlap
  (params (OtherActor :type Actor%20Object%20Reference)))

(event EventTick
  (params (DeltaSeconds :type Float%20%28single-precision%29)))

(event EventPlayAction
  (bind _receving_player (Variables|Default|GetReceving%20Player))
  (bind _returnvalue (Actor|GetComponentbyClass _receving_player "/Game/Virtuale/Blueprints/Components/Inventory.Inventory_C"))
  (if (Utilities|IsValid _returnvalue)
    (Utilities|Array|Add (Variables|/Game/Virtuale/Blueprints/Components/Inventory.Inventory_C|GetItems _returnvalue) (Variables|Default|GetObject))
    (CallFunction|EndAction true)
    (else
      (CallFunction|EndAction false))))

(fn ConstructionScript
  (|CallParentFunction))