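; BP_Action_Animate is an action that tells its source puppet to play a tagged animation at the target panel.
; It binds AttackHit to the puppet component's animation event, when that component exists, and sends AnimatePuppetMessage either way.
; EndAction fires immediately after the message and again from AttackHit, which unbinds itself, or straight away when no component exists.
; SetupAction and NewFunction are empty.
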(event Custom|AttackHit
  (params (AnimatingActor :type Actor%20Object%20Reference) (Animation :type Gameplay%20Tag%20Structure))
  (EventDispatchers|UnbindEventfromOnAnimationEvent (Actor|GetComponentbyClass (Variables|Default|GetSourcePuppet) "/Game/AdvancedTurnBasedTileToolkit/Core/Units/BP_PuppetComponent.BP_PuppetComponent_C") (delegate Custom|AttackHit))
  (CallFunction|EndAction true))

(event EventPlayAction
  (bind _sourcepuppet (Variables|Default|GetSourcePuppet))
  (bind _returnvalue (Actor|GetComponentbyClass _sourcepuppet "/Game/AdvancedTurnBasedTileToolkit/Core/Units/BP_PuppetComponent.BP_PuppetComponent_C"))
  (Utilities|IsValid _returnvalue
    (:Is%20Valid
      (EventDispatchers|BindEventtoOnAnimationEvent _returnvalue (delegate Custom|AttackHit))
      (Class|BPIPuppet|AnimatePuppet(Message) (Variables|Default|GetSourcePuppet) (Variables|Default|GetAnimTag) (Variables|Default|GetTargetPanel) "NewEnumerator0" :!label _label)
      (CallFunction|EndAction true))
    (:Is%20Not%20Valid
      (Utilities|FlowControl|Sequence
        (:then_0
          (goto _label))
        (:then_1
          (CallFunction|EndAction true))))))

(event EventSetupAction)

(fn ConstructionScript
  (|CallParentFunction))

(fn NewFunction
  (params (Target :type BP%20Unlockable%20Object%20Reference)))