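; Top-down style camera actor for controlling BP_Operative units, with panning, yaw rotation and clamped spring-arm zoom.
; It defaults to the first operative found and tracks its XY position while FollowOperative is set; manual movement clears that flag.
; Clicks sphere-trace from the camera against pawns, either selecting the hit operative or sending the current one to the clicked location through AI SimpleMoveToLocation.
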(event EventTick
  (params (DeltaSeconds :type Float%20%28single-precision%29))
  (bind _operative (Variables|Default|GetOperative))
  (bind _returnvalue (Transformation|GetActorLocation _operative))
  (if (Variables|Default|GetFollowOperative)
    (Transformation|SetActorLocation (Math|Vector|MakeVector (.x _returnvalue) (.y _returnvalue) (.z (Transformation|GetActorLocation))) false false)))

(event EventBeginPlay
  (bind _outactors (Actor|GetAllActorsOfClass "/Game/Virtuale/Blueprints/Operatives/BP_Operative.BP_Operative_C"))
  (Variables|Default|SetOperative (Utilities|Array|Get(acopy) _outactors)))

(fn ConstructionScript)

(fn Move
  (params (Direction :type Vector) (MovementSpeed :type Float%20%28double-precision%29))
  (Variables|Default|SetFollowOperative false)
  (Transformation|SetActorLocation (+ (* (Math|Vector|Normalize (+ (* (Transformation|GetActorRightVector) (.y Direction)) (* (Transformation|GetActorForwardVector) (.x Direction)))) MovementSpeed) (Transformation|GetActorLocation)) false false))

(fn Rotate
  (params (Direction :type Float%20%28double-precision%29) (RotationSpeed :type Float%20%28double-precision%29))
  (bind _returnvalue (Transformation|GetActorRotation))
  (Transformation|SetActorRotation (Math|Rotator|MakeRotator (.roll _returnvalue) (.pitch _returnvalue) (+ (* Direction RotationSpeed) (.yaw _returnvalue)))))

(fn Select/MoveOperative
  (params (MouseClickLocation :type Vector))
  (bind _outhit (Collision|SphereTraceForObjects (Transformation|GetWorldLocation (Variables|Default|GetCamera)) MouseClickLocation 1.0 (Utilities|Array|MakeArray "ObjectTypeQuery3") false 0 "ForDuration"))
  (bind _asbp_operative (Utilities|Casting|CastToBP_Operative (.HitActor (Collision|BreakHitResult _outhit)))
    (:then
      (Variables|Default|SetOperative _asbp_operative))
    (:CastFailed
      (AI|Navigation|SimpleMovetoLocation (AI|GetAIController (Variables|Default|GetOperative)) MouseClickLocation))))

(fn Zoom
  (params (Direction :type Float%20%28double-precision%29))
  (bind _springarm (Variables|Default|GetSpringArm))
  (Variables|/Script/Engine.SpringArmComponent|SetTargetArmLength _springarm (Math|Float|Min(Float) (Math|Float|Max(Float) (+ (* Direction 1e+02) (Variables|/Script/Engine.SpringArmComponent|GetTargetArmLength _springarm)) (Variables|Default|GetMiniminCameraZoom)) (Variables|Default|GetMaximumCameraZoom))))