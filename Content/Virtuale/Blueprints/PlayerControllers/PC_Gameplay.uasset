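; Gameplay player controller that turns Enhanced Input actions into commands for the possessed BP_Camera pawn.
; Movement and rotation inputs pass through helper functions that apply the controller's camera speeds.
; A click sends the world location under the cursor to the camera to select or move operatives.
; Other inputs zoom the camera, switch it to following an operative, or cycle to the next operative.
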(event Input|EnhancedActionEvents|EnhancedInputActionIA_CameraMovement
  (params (ActionValue :type Vector%202D%20Structure) (ElapsedSeconds :type Float%20%28double-precision%29) (TriggeredSeconds :type Float%20%28double-precision%29) (InputAction :type Input%20Action%20Object%20Reference :default "/Game/TopDown/Input/Actions/IA_CameraMovement.IA_CameraMovement"))
  (:Triggered
    (CallFunction|MoveCamera ActionValue :!label _label))
  (:Ongoing
    (goto _label)))

(event Input|EnhancedActionEvents|EnhancedInputActionIA_CameraRotation
  (params (ActionValue :type Float%20%28double-precision%29) (ElapsedSeconds :type Float%20%28double-precision%29) (TriggeredSeconds :type Float%20%28double-precision%29) (InputAction :type Input%20Action%20Object%20Reference :default "/Game/TopDown/Input/Actions/IA_CameraRotation.IA_CameraRotation"))
  (:Triggered
    (CallFunction|RotateCamera ActionValue :!label _label))
  (:Ongoing
    (goto _label)))

(event Input|EnhancedActionEvents|EnhancedInputActionIA_SetDestination_Click
  (params (ActionValue :type Boolean) (ElapsedSeconds :type Float%20%28double-precision%29) (TriggeredSeconds :type Float%20%28double-precision%29) (InputAction :type Input%20Action%20Object%20Reference :default "/Game/TopDown/Input/Actions/IA_SetDestination_Click.IA_SetDestination_Click"))
  (:Completed
    (CallFunction|ClickinWorld (.Location (CallFunction|GetLocationUnderCursor)))))

(event Input|EnhancedActionEvents|EnhancedInputActionIA_ToggleFollowOperative
  (params (ActionValue :type Boolean) (ElapsedSeconds :type Float%20%28double-precision%29) (TriggeredSeconds :type Float%20%28double-precision%29) (InputAction :type Input%20Action%20Object%20Reference :default "/Game/TopDown/Input/Actions/IA_ToggleFollowOperative.IA_ToggleFollowOperative"))
  (bind _asbp_camera (Utilities|Casting|CastToBP_Camera (Pawn|GetControlledPawn)))
  (Variables|/Game/Virtuale/Blueprints/BP_Camera.BP_Camera_C|SetFollowOperative _asbp_camera true))

(event Input|EnhancedActionEvents|EnhancedInputActionIA_CameraZoom
  (params (ActionValue :type Float%20%28double-precision%29) (ElapsedSeconds :type Float%20%28double-precision%29) (TriggeredSeconds :type Float%20%28double-precision%29) (InputAction :type Input%20Action%20Object%20Reference :default "/Game/TopDown/Input/Actions/IA_CameraZoom.IA_CameraZoom"))
  (bind _asbp_camera (Utilities|Casting|CastToBP_Camera (Pawn|GetControlledPawn)))
  (Default|Zoom _asbp_camera ActionValue))

(event Input|EnhancedActionEvents|EnhancedInputActionIA_SwapOperative
  (params (ActionValue :type Boolean) (ElapsedSeconds :type Float%20%28double-precision%29) (TriggeredSeconds :type Float%20%28double-precision%29) (InputAction :type Input%20Action%20Object%20Reference :default "/Game/TopDown/Input/Actions/IA_SwapOperative.IA_SwapOperative"))
  (:Completed
    (bind _asbp_camera (Utilities|Casting|CastToBP_Camera (Pawn|GetControlledPawn)))
    (Default|NextOperative _asbp_camera)))

(fn ConstructionScript
  (|CallParentFunction))

(fn MoveCamera
  (params (Direction :type Vector%202D%20Structure))
  (bind _asbp_camera (Utilities|Casting|CastToBP_Camera (Pawn|GetControlledPawn)))
  (Default|Move _asbp_camera (Math|Conversions|ToVector(Vector2D) Direction) (Variables|Default|GetCameraMovementSpeed)))

(fn RotateCamera
  (params (Direction :type Float%20%28double-precision%29))
  (bind _asbp_camera (Utilities|Casting|CastToBP_Camera (Pawn|GetControlledPawn)))
  (Default|Rotate _asbp_camera Direction (Variables|Default|GetCameraRotationSpeed)))

(fn ClickinWorld
  (params (Location :type Vector))
  (bind _asbp_camera (Utilities|Casting|CastToBP_Camera (Pawn|GetControlledPawn)))
  (Default|Select/MoveOperative _asbp_camera Location))