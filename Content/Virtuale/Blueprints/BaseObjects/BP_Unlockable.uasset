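; BP_Unlockable is a base object for things that open with a matching key.
; A key attempt compares the key to LockType, then calls an enact hook on a match or a failure hook otherwise.
; The check exists as both an event and a function, each with its own empty hooks.
; GetGridIndex is a stub that reports no valid grid position.
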(event Custom|KeyAttempt_Event
  (params (Key :type Enum_KeyTypes%20Enum :default "NewEnumerator0"))
  ;[1 1 1] We may want to add a bit of randomness
  (if (Utilities|Enum|Equal(Enum) Key (Variables|Default|GetLock%20Type))
    (CallFunction|EnactEventEvent)
    (else
      (CallFunction|FailEvent))))

(event Custom|EnactEvent_Event)

(event Custom|Fail_Event)

(fn ConstructionScript)

(fn GetGridIndex
  (return false 0))

(fn KeyAttempt
  (params (Key :type Enum_KeyTypes%20Enum :default "NewEnumerator0"))
  (if (Utilities|Enum|Equal(Enum) Key (Variables|Default|GetLock%20Type))
    (CallFunction|Enact)
    (return)
    (else
      (CallFunction|Failure)
      (return))))

(fn Enact)

(fn Failure)