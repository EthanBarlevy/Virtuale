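; Heart Stopper ability Blueprint for a grid-based game, containing targeting rules but no effect logic of its own.
; CheckRequirements defers to the parent, while CheckIfValidTarget adds a lookup of the clicked index in the grid manager's unit map.
; The target's current effect must equal two different enum values at once, so as written no target ever passes.
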(event EventBeginPlay
  (|CallParentFunction) ; This node is disabled and will not be called.\nDrag off pins to build functionality.
)

(event Collision|EventActorBeginOverlap
  (params (OtherActor :type Actor%20Object%20Reference)))

(event EventTick
  (params (DeltaSeconds :type Float%20%28single-precision%29)))

(fn ConstructionScript
  (|CallParentFunction))

(fn CheckRequirements
  (params (ActivatingActor :type Actor%20Object%20Reference))
  (bind _bmeetsrequirements (|CallParentFunction ActivatingActor))
  (return _bmeetsrequirements))

(fn CheckifValidTarget
  (params (ClickedIndex :type Integer%20%28by%20ref%29))
  (bind _gridmanagerref (Variables|Default|GetGridManagerRef))
  (bind _gridunits (Variables|/Game/AdvancedTurnBasedTileToolkit/Core/Grid/BP_GridManager.BP_GridManager_C|GetGridUnits _gridmanagerref))
  (bind (_value _returnvalue) (Utilities|Map|Find _gridunits ClickedIndex))
  (bind _currenteffect (Variables|/Game/AdvancedTurnBasedTileToolkit/Core/Units/BP_Unit.BP_Unit_C|GetCurrentEffect _value))
  (bind _bvalid (|CallParentFunction ClickedIndex))
  (return (Math|Boolean|ANDBoolean _bvalid _returnvalue (Utilities|Enum|Equal(Enum) (.effect _currenteffect) "NewEnumerator3") (Utilities|Enum|Equal(Enum) (.effect _currenteffect) "NewEnumerator2"))))