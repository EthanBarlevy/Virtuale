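; Scopeshot ability for John, described as using his scoped pistol to dispatch guards from range.
; Overrides GetDescription to supply its own name text while keeping the parent's description.
; On ExecuteAbility, an owner tagged John randomly adds one of two audio components or none, then the parent implementation handles the ability itself.
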(event EventBeginPlay
  (|CallParentFunction) ; This node is disabled and will not be called.\nDrag off pins to build functionality.
)

(event Collision|EventActorBeginOverlap
  (params (OtherActor :type Actor%20Object%20Reference)))

(event EventTick
  (params (DeltaSeconds :type Float%20%28single-precision%29)))

(fn ConstructionScript
  (|CallParentFunction))

(fn NewFunction0)

(fn GetDescription
  (bind _description (|CallParentFunction))
  (return "Scopeshot 
-- 
John uses his scoped pistol 
to dispatch guards from a range." _description))

(fn ExecuteAbility
  (params (TargetIndexIn :type Integer))
  (Utilities|FlowControl|Sequence
    (:then_0
      (if (Actor|ActorHasTag (Variables|Default|GetOwningActor) "John")
        (switch int (Math|Random|RandomInteger 3)
          (:0
            (AddComponent|AddAudioComponent false))
          (:1
            (AddComponent|AddAudioComponent false)))))
    (:then_1
      (bind _bsuccess (|CallParentFunction TargetIndexIn))
      (return _bsuccess))))