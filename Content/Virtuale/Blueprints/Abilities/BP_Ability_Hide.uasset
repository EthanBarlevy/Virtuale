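; Hide ability for a grid-based unit, triggered immediately on default click or by a primary-click server interaction through the default execution path.
; Execution spawns a BP_Action_Animate with the Anim.Hide tag on the owning unit's puppet and sets that unit's CurrentEffect.
; Target validation always passes, leaving an unlockable-object check unreachable.
; The description text is about hacking, despite the Hide name.
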(event EventServerInteract
  (params (bValidTile :type Boolean) (ClickedIndex :type Integer) (Location :type Vector :default "0, 0, 0") (Key :type Key%20Structure :default "None") (bReleased :type Boolean) (ClickType :type EClickType%20Enum :default "NewEnumerator0") (CallingPc :type BP%20Player%20Controller%20ATBTT%20Object%20Reference))
  (|CallParentFunction bValidTile ClickedIndex Location Key bReleased ClickType CallingPc)
  (if (and bValidTile (not bReleased))
    (switch Utilities|FlowControl|Switch|SwitchonEClickType ClickType
      (:NewEnumerator0
        (CallFunction|RunDefaultAbilityExecution (Variables|Default|GetClickedIndex))))))

(event Collision|EventActorBeginOverlap
  (params (OtherActor :type Actor%20Object%20Reference)))

(event EventTick
  (params (DeltaSeconds :type Float%20%28single-precision%29)))

(event EventBeginPlay
  (|CallParentFunction) ; This node is disabled and will not be called.\nDrag off pins to build functionality.
)

(fn ConstructionScript
  (|CallParentFunction))

(fn ExecuteAbility
  (params (TargetIndexIn :type Integer))
  (Game|SpawnActorfromClass "/Game/Virtuale/Blueprints/Actions/BP_Action_Animate.BP_Action_Animate_C" (Math|Transform|MakeTransform "0, 0, 0" "0, 0, 0" "1.000000,1.000000,1.000000") "Undefined" "MultiplyWithRoot" 0 "0.000000,0.000000,0.000000" "(TagName=\"Anim.Hide\")" (Variables|/Game/AdvancedTurnBasedTileToolkit/Core/Units/BP_Unit.BP_Unit_C|GetPuppet (Variables|Default|GetOwningUnit)) "NewEnumerator7" -1.0 "NewEnumerator0" 0)
  (Variables|/Game/AdvancedTurnBasedTileToolkit/Maps/Experimental/StatSystem/Units/BP_Unit_Stats_Anim.BP_Unit_Stats_Anim_C|SetCurrentEffect (Variables|Default|GetOwningUnit) (Utilities|Struct|MakeST_StatusEffect 0 0 "NewEnumerator1"))
  (return true))

(fn DefaultClick
  (params (GridIndex :type Integer%20%28by%20ref%29) (Location :type Vector :default "0, 0, 0"))
  (|CallParentFunction GridIndex Location)
  (CallFunction|ExecuteAbility)
  (return))

(fn CheckifValidTarget
  (params (ClickedIndex :type Integer%20%28by%20ref%29))
  (return true))

(fn GetDescription
  (return "Hide" "Hacking is the act of manipulating computer systems or networks to gain unauthorized access or exploit vulnerabilities."))