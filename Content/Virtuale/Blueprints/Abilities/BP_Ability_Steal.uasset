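; Steal ability for a grid-based unit, meant to target tiles holding a BP_Unlockable, though it only plays an animation.
; A server primary click on a valid tile runs default execution, while DefaultClick calls ExecuteAbility directly; execution spawns a BP_Action_Animate with the steal tag on the owning puppet.
; Requirements always pass, and target validation decides on the tile's first object only.
; Its description text describes hacking rather than stealing.
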(event EventServerInteract
  (params (bValidTile :type Boolean) (ClickedIndex :type Integer) (Location :type Vector :default "0, 0, 0") (Key :type Key%20Structure :default "None") (bReleased :type Boolean) (ClickType :type EClickType%20Enum :default "NewEnumerator0") (CallingPc :type BP%20Player%20Controller%20ATBTT%20Object%20Reference))
  (|CallParentFunction bValidTile ClickedIndex Location Key bReleased ClickType CallingPc)
  (if (and bValidTile (not bReleased))
    (switch Utilities|FlowControl|Switch|SwitchonEClickType ClickType
      (:NewEnumerator0
        (CallFunction|RunDefaultAbilityExecution (Variables|Default|GetClickedIndex))))))

(event Collision|EventActorBeginOverlap
  (params (OtherActor :type Actor%20Object%20Reference)))

(event EventTick
  (params (DeltaSeconds :type Float%20%28single-precision%29)))

(event EventBeginPlay
  (|CallParentFunction) ; This node is disabled and will not be called.\nDrag off pins to build functionality.
)

(fn ConstructionScript
  (|CallParentFunction))

(fn ExecuteAbility
  (params (TargetIndexIn :type Integer))
  (Game|SpawnActorfromClass "/Game/Virtuale/Blueprints/Actions/BP_Action_Animate.BP_Action_Animate_C" (Math|Transform|MakeTransform "0, 0, 0" "0, 0, 0" "1.000000,1.000000,1.000000") "Undefined" "MultiplyWithRoot" 0 "0.000000,0.000000,0.000000" "(TagName=\"Anim.Steal\")" (Variables|/Game/AdvancedTurnBasedTileToolkit/Core/Units/BP_Unit.BP_Unit_C|GetPuppet (Variables|Default|GetOwningUnit)) "NewEnumerator7" -1.0 "NewEnumerator0" 0)
  (return true))

(fn DefaultClick
  (params (GridIndex :type Integer%20%28by%20ref%29) (Location :type Vector :default "0, 0, 0"))
  (|CallParentFunction GridIndex Location)
  (CallFunction|ExecuteAbility)
  (return))

(fn CheckRequirements
  (params (ActivatingActor :type Actor%20Object%20Reference))
  (return true))

(fn CheckifValidTarget
  (params (ClickedIndex :type Integer%20%28by%20ref%29))
  (for _array_element (Utilities|Struct|BreakFObjects (.Value (Utilities|Map|Find (Variables|/Game/AdvancedTurnBasedTileToolkit/Core/Grid/BP_GridManager.BP_GridManager_C|GetGridObjects (Variables|Default|GetGridManagerRef)) ClickedIndex)))
    (Utilities|Casting|CastToBP_Unlockable _array_element
      (:then
        (return true))
      (:CastFailed
        (return false))))
  (return false))

(fn GetDescription
  (return "Steal" "Hacking is the act of manipulating computer systems or networks to gain unauthorized access or exploit vulnerabilities."))