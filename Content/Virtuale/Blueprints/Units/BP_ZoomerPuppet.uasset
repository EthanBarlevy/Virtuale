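; BP_ZoomerPuppet is a puppet version of the Zoomer unit that is rendered in isolation by a scene capture.
; On BeginPlay, its SceneCaptureComponent2D is restricted to showing only the puppet's own components.
; The Candy function toggles the Candyeating flag and sets the Weapon static mesh to candy or clears it.
; The construction script defers to the parent class.
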(event EventBeginPlay
  (Rendering|SceneCapture|ShowOnlyActorComponents (Variables|Default|GetSceneCaptureComponent2D) self false))

(event EventDestroyed)

(fn ConstructionScript
  (|CallParentFunction))

(fn Candy
  (bind _weapon (Variables|Default|GetWeapon))
  (bind _output_get (Variables|Default|Setcandyeating (not (Variables|Default|Getcandyeating))))
  (if _output_get
    (Components|StaticMesh|SetStaticMesh _weapon "/Game/Virtuale/Models/candy.candy")
    (else
      (Components|StaticMesh|SetStaticMesh _weapon 0))))