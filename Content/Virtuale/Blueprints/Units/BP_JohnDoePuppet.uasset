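; BP_JohnDoePuppet is a character puppet Blueprint that toggles cosmetic props on its mesh components.
; AddHat flips IsHiding and sets or clears the hat mesh on AdditionalProp.
; WeaponSwap flips HasWeapon and sets or clears the weapon mesh, with only the Pistol case mapped, to a scoped pistol.
; The event graph and construction script add no logic of their own.
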(event EventBeginPlay
  (|CallParentFunction) ; This node is disabled and will not be called.\nDrag off pins to build functionality.
)

(event Collision|EventActorBeginOverlap
  (params (OtherActor :type Actor%20Object%20Reference)))

(event EventTick
  (params (DeltaSeconds :type Float%20%28single-precision%29)))

(fn ConstructionScript
  (|CallParentFunction))

(fn AddHat
  (bind _additionalprop (Variables|Default|GetAdditionalProp))
  (bind _output_get (Variables|Default|SetIsHiding (not (Variables|Default|GetIsHiding))))
  (if _output_get
    (Components|StaticMesh|SetStaticMesh _additionalprop "/Game/Virtuale/Models/hat.hat")
    (else
      (Components|StaticMesh|SetStaticMesh _additionalprop 0))))

(fn WeaponSwap
  (params (Weapon :type E_WeaponType%20Enum :default "NewEnumerator7"))
  (bind _output_get (Variables|Default|SethasWeapon (not (Variables|Default|GethasWeapon))))
  (if _output_get
    (switch Utilities|FlowControl|Switch|SwitchonE_WeaponType Weapon
      (:NewEnumerator0
        (Components|StaticMesh|SetStaticMesh (Variables|Default|GetWeapon) "/Game/Virtuale/Models/scoped-pistol.scoped-pistol")))
    (else
      (Components|StaticMesh|SetStaticMesh (Variables|Default|GetWeapon) 0))))