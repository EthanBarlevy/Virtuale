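; Grid teleport point that moves a unit entering its tile to a paired teleporter's tile.
; On BeginPlay or UpdateFix it binds to the grid manager's tile-enter event and, once grid setup finishes, adds a pathfinding edge to the partner.
; If the destination is unoccupied, it relocates the unit on the grid, spawns a stairs-teleport action for the puppet and flags the unit to skip its next move action.
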(event Custom|Teleport
  (params (Unit :type BP%20Unit%20Object%20Reference) (GridIndex :type Integer))
  (if (== GridIndex (Variables|Default|GetGridIndex))
    (if (not (Utilities|Map|Contains (Variables|/Game/AdvancedTurnBasedTileToolkit/Core/Grid/BP_GridManager.BP_GridManager_C|GetGridUnits (Variables|Default|GetGridManagerRef)) (Variables|/Game/AdvancedTurnBasedTileToolkit/Core/Grid/BP_GridActor.BP_GridActor_C|GetGridIndex (Variables|teliport|GetPaired%20Teleporter))))
      (Default|TeleportUnitonGrid (Variables|Default|GetGridManagerRef) (Variables|/Game/AdvancedTurnBasedTileToolkit/Core/Grid/BP_GridActor.BP_GridActor_C|GetGridIndex (Variables|teliport|GetPaired%20Teleporter)) Unit)
      (Game|SpawnActorfromClass "/Game/Virtuale/Blueprints/Objects/BP_Action_StairsTeleport.BP_Action_StairsTeleport_C" (Math|Transform|MakeTransform "0, 0, 0" "0, 0, 0" "1.000000,1.000000,1.000000") "Undefined" "MultiplyWithRoot" 0 (Variables|/Game/AdvancedTurnBasedTileToolkit/Core/Units/BP_Unit.BP_Unit_C|GetPuppet Unit) (Transformation|GetWorldLocation (Variables|/Game/AdvancedTurnBasedTileToolkit/Core/Grid/BP_GridActor.BP_GridActor_C|GetBP_GridAnchor (Variables|teliport|GetPaired%20Teleporter))) (Variables|Default|GetVirtuále_Boom) (Variables|bp_TeleportPoint_C|GetVirtuále_Boom (Variables|teliport|GetPaired%20Teleporter)) -1.0 "NewEnumerator0" 0)
      (bind _asbp_unit_stats_anim (Utilities|Casting|CastToBP_Unit_Stats_Anim Unit))
      (Variables|/Game/AdvancedTurnBasedTileToolkit/Maps/Experimental/StatSystem/Units/BP_Unit_Stats_Anim.BP_Unit_Stats_Anim_C|SetbSkipNextMoveAction _asbp_unit_stats_anim true))))

(event EventBeginPlay
  (EventDispatchers|BindEventtoOnUnitEnterTileSimulate (Variables|Default|GetGridManagerRef) (delegate Custom|Teleport))
  (Utilities|DelayWhile (not (Variables|/Game/AdvancedTurnBasedTileToolkit/Core/Grid/BP_GridManager.BP_GridManager_C|GetbGridSetupDone (Variables|Default|GetGridManagerRef)))
    (:Continue
      (Default|AddEdge (Variables|Default|GetGridManagerRef) (Variables|Default|GetGridIndex) (Variables|/Game/AdvancedTurnBasedTileToolkit/Core/Grid/BP_GridActor.BP_GridActor_C|GetGridIndex (Variables|teliport|GetPaired%20Teleporter)) 1))))

(event EventUpdateFix
  (EventDispatchers|BindEventtoOnUnitEnterTileSimulate (Variables|Default|GetGridManagerRef) (delegate Custom|Teleport))
  (Utilities|DelayWhile (not (Variables|/Game/AdvancedTurnBasedTileToolkit/Core/Grid/BP_GridManager.BP_GridManager_C|GetbGridSetupDone (Variables|Default|GetGridManagerRef)))
    (:Continue
      (Default|AddEdge (Variables|Default|GetGridManagerRef) (Variables|Default|GetGridIndex) (Variables|/Game/AdvancedTurnBasedTileToolkit/Core/Grid/BP_GridActor.BP_GridActor_C|GetGridIndex (Variables|teliport|GetPaired%20Teleporter)) 1))))

(fn ConstructionScript)