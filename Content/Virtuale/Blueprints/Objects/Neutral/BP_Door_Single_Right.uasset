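; BP_Door_Single_Right is a single right-hand door actor that swings between open and closed rotations.
; On BeginPlay it waits ten seconds, sets Open and calls OpenCloseDoor, so the door opens by itself.
; OpenCloseDoor snaps the Door component's relative yaw to OpenRotation or ClosedRotation based on the Open flag, with no animation.
; Nothing in these graphs closes it again or reacts to overlaps.
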(event EventBeginPlay
  (Utilities|FlowControl|Delay 1e+01)
  (Variables|Default|SetOpen true)
  (CallFunction|Open|CloseDoor))

(event Collision|EventActorBeginOverlap
  (params (OtherActor :type Actor%20Object%20Reference)))

(event EventTick
  (params (DeltaSeconds :type Float%20%28single-precision%29)))

(fn ConstructionScript)

(fn Open|CloseDoor
  (if (Variables|Default|GetOpen)
    (Transformation|SetRelativeRotation (Variables|Default|GetDoor) (Math|Rotator|MakeRotator 0.0 0.0 (LocalVariables|GetOpen%20Rotation)) false false)
    (else
      (Transformation|SetRelativeRotation (Variables|Default|GetDoor) (Math|Rotator|MakeRotator 0.0 0.0 (LocalVariables|GetClosed%20Rotation)) false false))))