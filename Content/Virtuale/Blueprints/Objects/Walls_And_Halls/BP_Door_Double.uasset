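; Double door Blueprint that opens or closes when interacted with or lockpicked, as a child of an interactable parent class.
; Enact toggles unlocked doors, while a locked door allows only one lockpick attempt with a 50% success chance, calling the parent on success.
; Separate timelines lerp each leaf between closed and open rotations.
; When the left leaf finishes moving, the GridManager updates tiles within range of the door.
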(event Custom|Open%20|%20Close
  (if (Variables|Default|GetOpen)
    (Variables|Default|SetOpen false)
    (Utilities|FlowControl|Sequence
      (:then_0
        ;[0.2934 1 0.1701] Open
        (bind _door (Timeline|Open%20Right%20Door PlayFromStart)
          (:Update
            (Transformation|SetRelativeRotation (Variables|Default|GetRight%20Door) (Math|Rotator|Lerp(Rotator) (Variables|Default|GetClosed%20Rotation%20R) (Variables|Default|GetOpen%20Rotation%20R) _door true) false false))))
      (:then_1
        (bind _door_2 (Timeline|Open%20Left%20Door PlayFromStart)
          (:Update
            (Transformation|SetRelativeRotation (Variables|Default|GetLeft%20Door) (Math|Rotator|Lerp(Rotator) (Variables|Default|GetClosed%20Rotation%20L) (Variables|Default|GetOpen%20Rotation%20L) _door_2 true) false false))
          (:Finished
            (Default|UpdateTilesinRange (.GridManager (CallFunction|GetGridManager)) 1 0 (Transformation|GetActorLocation) false false true :!label _label)))))
    (else
      (Variables|Default|SetOpen true)
      (Utilities|FlowControl|Sequence
        (:then_0
          ;[1 0.1631 0.08678] Close
          (bind _door_3 (Timeline|Close%20Left%20Door PlayFromStart)
            (:Update
              (Transformation|SetRelativeRotation (Variables|Default|GetLeft%20Door) (Math|Rotator|Lerp(Rotator) (Variables|Default|GetOpen%20Rotation%20L) (Variables|Default|GetClosed%20Rotation%20L) _door_3 true) false false))
            (:Finished
              (goto _label))))
        (:then_1
          (bind _door_4 (Timeline|Close%20Right%20Door PlayFromStart)
            (:Update
              (Transformation|SetRelativeRotation (Variables|Default|GetRight%20Door) (Math|Rotator|Lerp(Rotator) (Variables|Default|GetOpen%20Rotation%20R) (Variables|Default|GetClosed%20Rotation%20R) _door_4 true) false false))))))))

(event EventBeginPlay
  (|CallParentFunction))

(event Collision|EventActorBeginOverlap
  (params (OtherActor :type Actor%20Object%20Reference)))

(event EventTick
  (params (DeltaSeconds :type Float%20%28single-precision%29)))

(fn ConstructionScript)

(fn Enact
  (params (KeyType :type Enum_KeyTypes%20Enum :default "NewEnumerator4"))
  (switch Utilities|FlowControl|Switch|SwitchonEnum_KeyTypes KeyType
    (:NewEnumerator1
      (if (Variables|Default|GetLocked)
        (if (Variables|Default|GetFirstLockpick)
          (Variables|Default|SetFirstLockpick false)
          (if (> (Math|Random|RandomFloat) 0.5)
            (CallFunction|Open|Close)
            (|CallParentFunction KeyType)))
        (else
          (CallFunction|Open|Close :!label _label)
          (|CallParentFunction KeyType))))
    (:NewEnumerator5
      (if (not (Variables|Default|GetLocked))
        (goto _label)))))