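; BP_Door_Single_Left is a lockable single door on the grid that swings open and closed via timelines.
; Enact handles Interact and Lockpick; the first lockpick has a 50% chance, later attempts always succeed.
; Materials show orange when locked and turn green once picked.
; Toggling or destruction swaps two collision volumes, refreshes nearby GridManager tiles and notifies I_UpdateFix actors; tiles refresh again when the swing finishes.
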(event Custom|Open%20|%20Close
  (if (Variables|Default|GetOpen)
    (Variables|Default|SetOpen false)
    (AddComponent|AddAudioComponent false)
    (CallFunction|ChangeActiveCollision)
    ;[0.2934 1 0.1701] Open
    (bind _door (Timeline|Open%20Door PlayFromStart)
      (:Update
        (Transformation|SetRelativeRotation (Variables|Default|GetDoor) (Math|Rotator|Lerp(Rotator) (Variables|Default|GetClosed%20Rotation) (Variables|Default|GetOpen%20Rotation) _door true) false false))
      (:Finished
        (Default|UpdateTilesinRange (.GridManager (CallFunction|GetGridManager)) 0 0 (Transformation|GetActorLocation) false false true :!label _label)))
    (else
      (Variables|Default|SetOpen true)
      (AddComponent|AddAudioComponent false)
      (CallFunction|ChangeActiveCollision)
      ;[1 0.1631 0.08678] Close
      (bind _door_2 (Timeline|Close%20Door PlayFromStart)
        (:Update
          (Transformation|SetRelativeRotation (Variables|Default|GetDoor) (Math|Rotator|Lerp(Rotator) (Variables|Default|GetOpen%20Rotation) (Variables|Default|GetClosed%20Rotation) _door_2 true) false false))
        (:Finished
          (goto _label))))))

(event EventBeginPlay
  (|CallParentFunction))

(event EventDestroyed
  (CallFunction|ChangeActiveCollision)
  (|CallParentFunction))

(fn ConstructionScript
  (bind _door (Variables|Default|GetDoor))
  (bind _door_wire (Variables|Default|GetDoor_Wire))
  (if (Variables|Default|GetLocked)
    (Rendering|Material|SetMaterial _door 0 "/Game/Virtuale/Shaders/Grids_and_Wires/M_Grid_Object_orange.M_Grid_Object_orange")
    (Rendering|Material|SetMaterial _door 1 "/Game/Virtuale/Shaders/Grids_and_Wires/M_Grid_Object_orange.M_Grid_Object_orange")
    (Rendering|Material|SetMaterial _door_wire 0 "/Game/Virtuale/Shaders/Grids_and_Wires/M_WireFrame_orange.M_WireFrame_orange")
    (Rendering|Material|SetMaterial _door_wire 1 "/Game/Virtuale/Shaders/Grids_and_Wires/M_WireFrame_orange.M_WireFrame_orange"))
  (|CallParentFunction))

(fn Enact
  (params (KeyType :type Enum_KeyTypes%20Enum :default "NewEnumerator4"))
  (bind _door (Variables|Default|GetDoor))
  (bind _door_wire (Variables|Default|GetDoor_Wire))
  (switch Utilities|FlowControl|Switch|SwitchonEnum_KeyTypes KeyType
    (:NewEnumerator1
      (if (Variables|Default|GetLocked)
        (if (Variables|Default|GetFirstLockpick)
          (Variables|Default|SetFirstLockpick false)
          (if (> (Math|Random|RandomFloat) 0.5)
            (Variables|Default|SetLocked false :!label _label)
            (Rendering|Material|SetMaterial _door 0 "/Game/Virtuale/Shaders/Grids_and_Wires/M_Grid_Object_green.M_Grid_Object_green")
            (Rendering|Material|SetMaterial _door 1 "/Game/Virtuale/Shaders/Grids_and_Wires/M_Grid_Object_green.M_Grid_Object_green")
            (Rendering|Material|SetMaterial _door_wire 0 "/Game/Virtuale/Shaders/Grids_and_Wires/M_WireFrame_green.M_WireFrame_green")
            (Rendering|Material|SetMaterial _door_wire 1 "/Game/Virtuale/Shaders/Grids_and_Wires/M_WireFrame_green.M_WireFrame_green")
            (CallFunction|Open|Close)
            (|CallParentFunction KeyType))
          (else
            (goto _label)))
        (else
          (CallFunction|Open|Close :!label _label_2)
          (|CallParentFunction "NewEnumerator4"))))
    (:NewEnumerator5
      (if (not (Variables|Default|GetLocked))
        (goto _label_2)))))

(fn ChangeActiveCollision
  (bind _opencollision (Variables|Default|GetOpenCollision))
  (bind _closecollision (Variables|Default|GetCloseCollision))
  (if (Variables|Default|GetOpen)
    (Collision|SetCollisionProfileName _opencollision "NoCollision" true :!class /Script/Engine.PrimitiveComponent)
    (Collision|SetCollisionProfileName _closecollision "BlockAllDynamic" true :!class /Script/Engine.PrimitiveComponent)
    (else
      (Collision|SetCollisionProfileName _opencollision "BlockAllDynamic" true :!class /Script/Engine.PrimitiveComponent)
      (Collision|SetCollisionProfileName _closecollision "NoCollision" true :!class /Script/Engine.PrimitiveComponent)))
  (Default|UpdateTilesinRange (.GridManager (CallFunction|GetGridManager)) 0 0 (Transformation|GetActorLocation) false false true)
  (bind _outactors (Actor|GetAllActorswithInterface "/Game/Virtuale/Blueprints/Objects/I_UpdateFix.I_UpdateFix_C"))
  (for _array_element _outactors
    (Class|IUpdateFix|UpdateFix(Message) _array_element)))