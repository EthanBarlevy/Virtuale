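; Right-hinged single door on the tactical grid that units open or close by interacting, or lockpick when locked.
; Lockpicking has a coin-flip first attempt and later always succeeds, with random voice lines from the nearest unit (John or Zoom).
; Timelines rotate the door, and material colors show lock state.
; Toggling or destruction updates collision, refreshes nearby GridManager tiles and notifies every I_UpdateFix actor.
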(event Custom|Open%20|%20Close
  (if (Variables|Default|GetOpen)
    (Variables|Default|SetOpen false)
    (AddComponent|AddAudioComponent false)
    (CallFunction|ChangeActiveCollision)
    ;[0.2934 1 0.1701] Open
    (bind _door (Timeline|Open%20Door PlayFromStart)
      (:Update
        (Transformation|SetRelativeRotation (Variables|Default|GetDoor) (Math|Rotator|Lerp(Rotator) (Variables|Default|GetClosed%20Rotation) (Variables|Default|GetOpen%20Rotation) _door true) false false))
      (:Finished
        (Default|UpdateTilesinRange (.GridManager (CallFunction|GetGridManager)) 0 0 (Transformation|GetActorLocation) false false true :!label _label)
        (bind _outactors (Actor|GetAllActorswithInterface "/Game/Virtuale/Blueprints/Objects/I_UpdateFix.I_UpdateFix_C"))
        (for _array_element _outactors
          (Class|IUpdateFix|UpdateFix(Message) _array_element))))
    (else
      (Variables|Default|SetOpen true)
      (AddComponent|AddAudioComponent false)
      (CallFunction|ChangeActiveCollision)
      ;[1 0.1631 0.08678] Comment
      (bind _door_2 (Timeline|Close%20Door PlayFromStart)
        (:Update
          (Transformation|SetRelativeRotation (Variables|Default|GetDoor) (Math|Rotator|Lerp(Rotator) (Variables|Default|GetOpen%20Rotation) (Variables|Default|GetClosed%20Rotation) _door_2 true) false false))
        (:Finished
          (goto _label))))))

(event EventBeginPlay
  (|CallParentFunction))

(event Collision|EventActorBeginOverlap
  (params (OtherActor :type Actor%20Object%20Reference)))

(event EventTick
  (params (DeltaSeconds :type Float%20%28single-precision%29)))

(event EventDestroyed
  (CallFunction|ChangeActiveCollision)
  (Utilities|FlowControl|Sequence
    (:then_0
      (Collision|SetCollisionProfileName (Variables|Default|GetCloseCollision) "NoCollision" true :!class /Script/Engine.PrimitiveComponent)
      (Collision|SetCollisionProfileName (Variables|Default|GetOpenCollision) "NoCollision" true :!class /Script/Engine.PrimitiveComponent))
    (:then_1
      (Default|UpdateTilesinRange (.GridManager (CallFunction|GetGridManager)) 1 0 (Transformation|GetActorLocation) false false true)
      (bind _outactors (Actor|GetAllActorswithInterface "/Game/Virtuale/Blueprints/Objects/I_UpdateFix.I_UpdateFix_C"))
      (for _array_element _outactors
        (Class|IUpdateFix|UpdateFix(Message) _array_element))
      (|CallParentFunction))))

(fn ConstructionScript
  (bind _door (Variables|Default|GetDoor))
  (bind _door_wire (Variables|Default|GetDoor_Wire))
  (if (Variables|Default|GetLocked)
    (Rendering|Material|SetMaterial _door 0 "/Game/Virtuale/Shaders/Grids_and_Wires/M_Grid_Object_orange.M_Grid_Object_orange")
    (Rendering|Material|SetMaterial _door 1 "/Game/Virtuale/Shaders/Grids_and_Wires/M_Grid_Object_orange.M_Grid_Object_orange")
    (Rendering|Material|SetMaterial _door_wire 0 "/Game/Virtuale/Shaders/Grids_and_Wires/M_WireFrame_orange.M_WireFrame_orange")
    (Rendering|Material|SetMaterial _door_wire 1 "/Game/Virtuale/Shaders/Grids_and_Wires/M_WireFrame_orange.M_WireFrame_orange"))
  (|CallParentFunction))

(fn Enact
  (params (KeyType :type Enum_KeyTypes%20Enum :default "NewEnumerator4"))
  (bind _door (Variables|Default|GetDoor))
  (bind _door_wire (Variables|Default|GetDoor_Wire))
  (switch Utilities|FlowControl|Switch|SwitchonEnum_KeyTypes KeyType
    (:NewEnumerator1
      (if (Variables|Default|GetLocked)
        (if (Variables|Default|GetFirstLockpick)
          (Variables|Default|SetFirstLockpick false)
          (if (> (Math|Random|RandomFloat) 0.5)
            (Variables|Default|SetLocked false :!label _label)
            (Utilities|FlowControl|Sequence
              (:then_0
                (bind _outactors (Actor|GetAllActorsOfClass "/Game/AdvancedTurnBasedTileToolkit/Maps/Experimental/StatSystem/Units/BP_Unit_Stats_Anim.BP_Unit_Stats_Anim_C" :!label _label_2))
                (for _array_element _outactors
                  (bind _gridindex (Default|GetGridIndex _array_element))
                  (if (< (Math|Vector|Distance(Vector) (Transformation|GetActorLocation) (.Value (Utilities|Map|Find (Variables|/Game/AdvancedTurnBasedTileToolkit/Core/Grid/BP_GridManager.BP_GridManager_C|GetGridLocations (.GridManager (CallFunction|GetGridManager))) _gridindex))) (LocalVariables|GetDistance))
                    (LocalVariables|SetDistance (Math|Vector|Distance(Vector) (Transformation|GetActorLocation) (.Value (Utilities|Map|Find (Variables|/Game/AdvancedTurnBasedTileToolkit/Core/Grid/BP_GridManager.BP_GridManager_C|GetGridLocations (.GridManager (CallFunction|GetGridManager))) _gridindex))))
                    (LocalVariables|SetActor _array_element)))
                (if (LocalVariables|GetPass|Fail)
                  (if (Actor|ActorHasTag (LocalVariables|GetActor) "John")
                    (switch int (Math|Random|RandomInteger 9)
                      (:0
                        (AddComponent|AddAudioComponent false))
                      (:1
                        (AddComponent|AddAudioComponent false))
                      (:2
                        (AddComponent|AddAudioComponent false)))
                    (elif (Actor|ActorHasTag (LocalVariables|GetActor) "Zoom")
                      (switch int (Math|Random|RandomInteger 7)
                        (:0
                          (AddComponent|AddAudioComponent false))
                        (:1
                          (AddComponent|AddAudioComponent false)))))
                  (elif (Actor|ActorHasTag (LocalVariables|GetActor) "John")
                    (switch int (Math|Random|RandomInteger 7)
                      (:0
                        (AddComponent|AddAudioComponent false))
                      (:1
                        (AddComponent|AddAudioComponent false)))
                    (elif (Actor|ActorHasTag (LocalVariables|GetActor) "Zoom")
                      (switch int (Math|Random|RandomInteger 9)
                        (:0
                          (AddComponent|AddAudioComponent false))
                        (:1
                          (AddComponent|AddAudioComponent false))
                        (:2
                          (AddComponent|AddAudioComponent false)))))))
              (:then_1
                (Rendering|Material|SetMaterial _door 0 "/Game/Virtuale/Shaders/Grids_and_Wires/M_Grid_Object_green.M_Grid_Object_green")
                (Rendering|Material|SetMaterial _door 1 "/Game/Virtuale/Shaders/Grids_and_Wires/M_Grid_Object_green.M_Grid_Object_green")
                (Rendering|Material|SetMaterial _door_wire 0 "/Game/Virtuale/Shaders/Grids_and_Wires/M_WireFrame_green.M_WireFrame_green")
                (Rendering|Material|SetMaterial _door_wire 1 "/Game/Virtuale/Shaders/Grids_and_Wires/M_WireFrame_green.M_WireFrame_green")
                (CallFunction|Open|Close)
                (|CallParentFunction KeyType)))
            (else
              (LocalVariables|SetPass|Fail false)
              (goto _label_2)))
          (else
            (goto _label)))
        (else
          (CallFunction|Open|Close :!label _label_3)
          (|CallParentFunction "NewEnumerator4"))))
    (:NewEnumerator5
      (if (not (Variables|Default|GetLocked))
        (goto _label_3)))))

(fn ChangeActiveCollision
  (bind _opencollision (Variables|Default|GetOpenCollision))
  (bind _closecollision (Variables|Default|GetCloseCollision))
  (if (Variables|Default|GetOpen)
    (Collision|SetCollisionProfileName _opencollision "NoCollision" true :!class /Script/Engine.PrimitiveComponent)
    (Collision|SetCollisionProfileName _closecollision "BlockAllDynamic" true :!class /Script/Engine.PrimitiveComponent)
    (else
      (Collision|SetCollisionProfileName _opencollision "BlockAllDynamic" true :!class /Script/Engine.PrimitiveComponent)
      (Collision|SetCollisionProfileName _closecollision "NoCollision" true :!class /Script/Engine.PrimitiveComponent)))
  (Default|UpdateTilesinRange (.GridManager (CallFunction|GetGridManager)) 0 0 (Transformation|GetActorLocation) false false true)
  (bind _outactors (Actor|GetAllActorswithInterface "/Game/Virtuale/Blueprints/Objects/I_UpdateFix.I_UpdateFix_C"))
  (for _array_element _outactors
    (Class|IUpdateFix|UpdateFix(Message) _array_element)))