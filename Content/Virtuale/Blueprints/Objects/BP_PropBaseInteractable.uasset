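; Base interactable grid prop with an optional key lock and the ability to switch between opaque and see-through.
; Key attempts route to empty Enact or Failure stubs, while allowed interactions remove the prop from the grid.
; Construction gathers static meshes as opaque when the prop sits above a height threshold; the translucent list is never filled.
; MakeTransparent and MakeOpaque pass through gates opened at BeginPlay to toggle mesh visibility and trace-channel blocking.
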(event Custom|KeyAttempt_Event
  (params (Key :type Enum_KeyTypes%20Enum :default "NewEnumerator0"))
  (bind _locktype (Variables|Default|GetLockType))
  ;[1 1 1] We may want to add a bit of randomness
  (if (Utilities|Enum|Equal(Enum) _locktype "NewEnumerator6")
    (CallFunction|Enact Key :!label _label)
    (elif (Utilities|Enum|Equal(Enum) Key _locktype)
      (goto _label)
      (else
        (CallFunction|Failure "NewEnumerator4")))))

(event Custom|MakeTransparent
  (Utilities|FlowControl|Gate true
    (:Exit
      (for _array_element (Variables|Default|GetOpaqueMeshes_0)
        (Rendering|SetVisibility _array_element false false)
        (Collision|SetCollisionResponsetoChannel _array_element "ECC_GameTraceChannel1" "ECR_Ignore")
        (for _array_element_2 (Variables|Default|GetTranslucentMeshes_0)
          (Rendering|SetVisibility _array_element_2 true false))))))

(event Custom|MakeOpaque
  (Utilities|FlowControl|Gate true
    (:Exit
      (for _array_element (Variables|Default|GetOpaqueMeshes_0)
        (Rendering|SetVisibility _array_element true false)
        (Collision|SetCollisionResponsetoChannel _array_element "ECC_GameTraceChannel1" "ECR_Block")
        (for _array_element_2 (Variables|Default|GetTranslucentMeshes_0)
          (Rendering|SetVisibility _array_element_2 false false))))))

(event EventInteract
  (params (TriggeringActor :type Actor%20Object%20Reference) (InteractionType :type Gameplay%20Tag%20Container%20Structure))
  (bind _ballowed (CallFunction|CheckifInteractionAllowed TriggeringActor InteractionType))
  (if _ballowed
    (if true
      (Default|RemoveObjectfromGrid (Variables|Default|GetGridManagerRef) self (Variables|Default|GetGridIndex)))))

(event EventBeginPlay
  (Utilities|FlowControl|Sequence
    (:then_0
      (Utilities|FlowControl|Gate true) ; enters at Open
    )
    (:then_1
      (Utilities|FlowControl|Gate true) ; enters at Open
    )
    (:then_2
      (|CallParentFunction))))

(fn ConstructionScript
  (if (> (.z (.location (Transformation|GetWorldTransform (Variables|Default|GetSceneComponent)))) 249.0)
    (Utilities|Array|Clear (Variables|Default|GetOpaqueMeshes_0))
    (Utilities|Array|Clear (Variables|Default|GetTranslucentMeshes_0))
    (for _array_element (Actor|GetComponentsByClass "/Script/Engine.StaticMeshComponent")
      (Utilities|Array|Add (Variables|Default|GetOpaqueMeshes_0) _array_element)))
  (|CallParentFunction))

(fn Enact
  (params (KeyType :type Enum_KeyTypes%20Enum :default "NewEnumerator4")))

(fn Failure
  (params (KeyType :type Enum_KeyTypes%20Enum :default "NewEnumerator4")))