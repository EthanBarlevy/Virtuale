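; Double-leaf gate that automatically swings open and closed on a looping five-second timer started at BeginPlay.
; Each toggle flips the Open flag and plays one timeline per leaf, lerping relative rotation of Left and Right between stored open and closed rotators along the shortest path.
; The flag reads inverted: when true, the gate animates toward open and the flag becomes false.
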(event Custom|Open%20|%20Close
  (if (Variables|Default|GetOpen)
    (Variables|Default|SetOpen false)
    (Utilities|FlowControl|Sequence
      (:then_0
        (bind _door (Timeline|Timeline_1 PlayFromStart)
          (:Update
            (Transformation|SetRelativeRotation (Variables|Default|GetRight) (Math|Rotator|Lerp(Rotator) (Variables|Default|GetClosed%20Rotation%20R) (Variables|Default|GetOpen%20Rotation%20R) _door true) false false))))
      (:then_1
        (bind _door_2 (Timeline|Timeline PlayFromStart)
          (:Update
            (Transformation|SetRelativeRotation (Variables|Default|GetLeft) (Math|Rotator|Lerp(Rotator) (Variables|Default|GetClosed%20Rotation%20L) (Variables|Default|GetOpen%20Rotation%20L) _door_2 true) false false)))))
    (else
      (Variables|Default|SetOpen true)
      (Utilities|FlowControl|Sequence
        (:then_0
          (bind _door_3 (Timeline|Timeline_0 PlayFromStart)
            (:Update
              (Transformation|SetRelativeRotation (Variables|Default|GetLeft) (Math|Rotator|Lerp(Rotator) (Variables|Default|GetOpen%20Rotation%20L) (Variables|Default|GetClosed%20Rotation%20L) _door_3 true) false false))))
        (:then_1
          (bind _door_4 (Timeline|Timeline_2 PlayFromStart)
            (:Update
              (Transformation|SetRelativeRotation (Variables|Default|GetRight) (Math|Rotator|Lerp(Rotator) (Variables|Default|GetOpen%20Rotation%20R) (Variables|Default|GetClosed%20Rotation%20R) _door_4 true) false false))))))))

(event Custom|Open%20/%20Close
  (CallFunction|Open|Close))

(event EventBeginPlay
  (Utilities|Time|SetTimerbyEvent (delegate Custom|Open%20/%20Close) 5.0 true))

(fn ConstructionScript)