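; Vault door that players open by hacking or lockpicking, awarding an achievement for either method.
; Enact opens it when a hack brings TimesHacked to one, or on a random lockpick roll whose small odds rise with TimesHacked.
; Open|Close waits briefly, then timelines lerp the door's rotation and location between closed and open transforms.
; When either animation finishes, the grid manager updates nearby tiles.
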(event Custom|Open%20|%20Close
  (bind _vault (Variables|Default|Getvault))
  (bind _vault_2 (Variables|Default|Getvault))
  (Utilities|FlowControl|Delay 0.5)
  (if (Variables|Default|GetOpen)
    (Variables|Default|SetOpen false)
    ;[0.2934 1 0.1701] Open
    (bind _door (Timeline|Open%20Valut PlayFromStart)
      (:Update
        (Transformation|SetRelativeRotation _vault (Math|Rotator|Lerp(Rotator) (Variables|Default|GetClosed%20Rotation) (Variables|Default|GetOpen%20Rotation) _door true) false false)
        (Transformation|SetRelativeLocation _vault (Math|Vector|Lerp(Vector) (Variables|Default|GetClosed%20Location) (Variables|Default|GetOpen%20Location) _door) false false))
      (:Finished
        (Default|UpdateTilesinRange (.GridManager (CallFunction|GetGridManager)) 1 0 (Transformation|GetActorLocation) false false true :!label _label)))
    (else
      (Variables|Default|SetOpen true)
      ;[1 0.1631 0.08678] Close
      (bind _door_2 (Timeline|Close%20Vault PlayFromStart)
        (:Update
          (Transformation|SetRelativeRotation _vault_2 (Math|Rotator|Lerp(Rotator) (Variables|Default|GetOpen%20Rotation) (Variables|Default|GetClosed%20Rotation) _door_2 true) false false)
          (Transformation|SetRelativeLocation _vault_2 (Math|Vector|Lerp(Vector) (Variables|Default|GetOpen%20Location) (Variables|Default|GetClosed%20Location) _door_2) false false))
        (:Finished
          (goto _label))))))

(fn ConstructionScript
  (|CallParentFunction))

(fn Enact
  (params (KeyType :type Enum_KeyTypes%20Enum :default "NewEnumerator4"))
  (bind _returnvalue (Math|Random|RandomFloat))
  (if (Variables|Default|GetOpen)
    (switch Utilities|FlowControl|Switch|SwitchonEnum_KeyTypes KeyType
      (:NewEnumerator4
        (|CallParentFunction "NewEnumerator4"))
      (:NewEnumerator0
        (bind _result (Math|Integer|IncrementInt (Variables|Default|GetTimesHacked))
          (:%20%20
            (if (== _result 1)
              (Default|CallOpenVault)
              (CallFunction|Open|Close)
              (Default|AchievementGet (.PlayerControllerATBTT (CallFunction|GetPlayerControllerATBTT)) "Hackerman"))
            (|CallParentFunction "NewEnumerator0"))))
      (:NewEnumerator1
        (switch int (Variables|Default|GetTimesHacked)
          (:0
            (if (> _returnvalue 0.99)
              (Default|CallOpenVault :!label _label)
              (CallFunction|Open|Close)
              (Default|AchievementGet (.PlayerControllerATBTT (CallFunction|GetPlayerControllerATBTT)) "Speedrun")
              (|CallParentFunction "NewEnumerator1")))
          (:1
            (if (> _returnvalue 0.95)
              (goto _label)))
          (:2
            (if (> _returnvalue 0.9)
              (goto _label)))
          (:3
            (if (> _returnvalue 0.85)
              (goto _label)))
          (:4
            (if (> _returnvalue 0.8)
              (goto _label))))))))

(fn Failure
  (params (KeyType :type Enum_KeyTypes%20Enum :default "NewEnumerator4"))
  (|CallParentFunction "NewEnumerator4"))