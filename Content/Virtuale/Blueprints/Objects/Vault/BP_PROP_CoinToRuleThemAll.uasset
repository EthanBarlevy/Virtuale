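; Vault coin prop that spins in place and grants loot when enacted.
; A looping Timeline drives the coin's yaw, restarting after a zero-length Delay each time it finishes.
; Enact casts the turn manager's active unit to BP_Unit_Stats_Anim, adds a "Rubber Duck" loot entry, calls Check on it, destroys the coin, then calls the parent Enact.
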(event EventBeginPlay
  (bind _yaw (Timeline|Timeline Play)
    (:Update
      (Transformation|SetRelativeRotation (Variables|Default|GetCoin) (Math|Rotator|MakeRotator 0.0 0.0 (* _yaw 15.0)) false false))
    (:Finished
      (Utilities|FlowControl|Delay 0.0)
      (Timeline|Timeline PlayFromStart))))

(fn ConstructionScript)

(fn Enact
  (params (KeyType :type Enum_KeyTypes%20Enum :default "NewEnumerator4"))
  (bind _asbp_unit_stats_anim (Utilities|Casting|CastToBP_Unit_Stats_Anim (Variables|/Game/AdvancedTurnBasedTileToolkit/Core/BP_TurnManager.BP_TurnManager_C|GetActiveUnit (.TurnManager (CallFunction|GetTurnManager)))))
  (Utilities|Array|Add (Variables|/Game/AdvancedTurnBasedTileToolkit/Maps/Experimental/StatSystem/Units/BP_Unit_Stats_Anim.BP_Unit_Stats_Anim_C|GetLoot _asbp_unit_stats_anim) (Utilities|Struct|MakeST_Loot "Rubber Duck" 1.0 0))
  (Default|Check _asbp_unit_stats_anim)
  (Actor|DestroyActor)
  (|CallParentFunction KeyType))