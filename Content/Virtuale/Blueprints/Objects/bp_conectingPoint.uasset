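; Grid connection point that links its tile to the tile of a paired connection by adding a pathing edge.
; On BeginPlay it hides its sphere, then runs the same setup as UpdateFix, waiting for the grid manager to finish setup before adding the cost-1 edge.
; It also binds Connect to the manager's simulated unit-enter-tile event, but that handler is empty.
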(event Custom|Connect
  (params (Unit :type BP%20Unit%20Object%20Reference) (GridIndex :type Integer)))

(event EventBeginPlay
  (Rendering|SetVisibility (Variables|Default|GetSphere) false false)
  (EventDispatchers|BindEventtoOnUnitEnterTileSimulate (Variables|Default|GetGridManagerRef) (delegate Custom|Connect))
  (Utilities|DelayWhile (not (Variables|/Game/AdvancedTurnBasedTileToolkit/Core/Grid/BP_GridManager.BP_GridManager_C|GetbGridSetupDone (Variables|Default|GetGridManagerRef)))
    (:Continue
      (Default|AddEdge (Variables|Default|GetGridManagerRef) (Variables|Default|GetGridIndex) (Variables|/Game/AdvancedTurnBasedTileToolkit/Core/Grid/BP_GridActor.BP_GridActor_C|GetGridIndex (Variables|teliport|GetPaired%20Conection)) 1))))

(event EventUpdateFix
  (EventDispatchers|BindEventtoOnUnitEnterTileSimulate (Variables|Default|GetGridManagerRef) (delegate Custom|Connect))
  (Utilities|DelayWhile (not (Variables|/Game/AdvancedTurnBasedTileToolkit/Core/Grid/BP_GridManager.BP_GridManager_C|GetbGridSetupDone (Variables|Default|GetGridManagerRef)))
    (:Continue
      (Default|AddEdge (Variables|Default|GetGridManagerRef) (Variables|Default|GetGridIndex) (Variables|/Game/AdvancedTurnBasedTileToolkit/Core/Grid/BP_GridActor.BP_GridActor_C|GetGridIndex (Variables|teliport|GetPaired%20Conection)) 1))))

(fn ConstructionScript)