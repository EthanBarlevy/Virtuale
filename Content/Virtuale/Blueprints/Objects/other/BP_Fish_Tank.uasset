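; Breakable fish tank object that spins its water disk every tick and leaves a fish prop behind when destroyed.
; On Destroyed it spawns the fish at the floor, disables water collision and refreshes nearby grid manager tiles.
; It then notifies every I_UpdateFix actor to update its fix message before running the parent's logic.
; A separate destroy event removes the actor after a short delay.
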(event Custom|destroy
  (Utilities|FlowControl|Delay 0.9)
  (Actor|DestroyActor))

(event EventDestroyed
  (Game|SpawnActorfromClass "/Game/Virtuale/Blueprints/Objects/other/BP_PROP_Fish.BP_PROP_Fish_C" (Math|Transform|MakeTransform (Transformation|GetWorldLocation (Variables|Default|Getfloor)) "-90.000000,0.000000,0.000000" "1.000000,1.000000,1.000000") "Undefined" "MultiplyWithRoot" 0 0)
  (Collision|SetCollisionEnabled (Variables|Default|Getwater) "NoCollision")
  (Default|UpdateTilesinRange (.GridManager (CallFunction|GetGridManager)) 1 0 (Transformation|GetActorLocation) false false true)
  (bind _outactors (Actor|GetAllActorswithInterface "/Game/Virtuale/Blueprints/Objects/I_UpdateFix.I_UpdateFix_C"))
  (for _array_element _outactors
    (Class|IUpdateFix|UpdateFix(Message) _array_element))
  (|CallParentFunction))

(event EventTick
  (params (DeltaSeconds :type Float%20%28single-precision%29))
  (Transformation|AddLocalRotation (Variables|Default|GetwaterDisk) (Math|Rotator|MakeRotator 0.0 0.0 (Variables|Default|GetRotation%20Speed)) false false))

(fn ConstructionScript)