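; C4 explosive actor that breaks a nearby destructible object when detonated.
; Detonate gathers actors carrying a destructible tag, finds the one nearest the C4 component and destroys it if it is within a short fixed radius, then destroys itself.
; The Blueprint has no active event logic, radial damage or effects, so Detonate relies on an external call.
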(event EventBeginPlay
  (|CallParentFunction) ; This node is disabled and will not be called.\nDrag off pins to build functionality.
)

(event Collision|EventActorBeginOverlap
  (params (OtherActor :type Actor%20Object%20Reference)))

(event EventTick
  (params (DeltaSeconds :type Float%20%28single-precision%29)))

(fn ConstructionScript
  (|CallParentFunction))

(fn Detonate
  (bind _outactors (Actor|GetAllActorswithTag "Blowthefuckupable"))
  (if (> (.Distance (Actor|FindNearestActor (Transformation|GetWorldLocation (Variables|Default|Getc4)) _outactors)) 1e+02)
    _
    (else
      (Actor|DestroyActor (.ReturnValue (Actor|FindNearestActor (Transformation|GetWorldLocation (Variables|Default|Getc4)) _outactors)))))
  (Actor|DestroyActor))