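; BP_The_Pool is a decorative pool object with a rubber duck that bobs and spins.
; On BeginPlay it stores the duck's starting height, and a Timeline lerps its Z around that height, replaying from the start whenever it finishes.
; Each Tick yaws the Center component and the duck at separate per-frame rates, unscaled by delta time.
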(event EventTick
  (params (DeltaSeconds :type Float%20%28single-precision%29))
  (Transformation|AddLocalRotation (Variables|Default|Getcenter) (Math|Rotator|MakeRotator 0.0 0.0 (Variables|Default|GetRotation%201)) false false)
  (Transformation|AddLocalRotation (Variables|Default|Getrubber_duck_pool) (Math|Rotator|MakeRotator 0.0 0.0 (Variables|Default|GetRotation%202)) false false))

(event EventBeginPlay
  (bind _rubber_duck_pool (Variables|Default|Getrubber_duck_pool))
  (bind _returnvalue (Transformation|GetWorldLocation _rubber_duck_pool))
  (|CallParentFunction)
  (Variables|Default|Setstarting%20Z (.z (Transformation|GetWorldLocation (Variables|Default|Getrubber_duck_pool))))
  (bind _newtrack_0 (Timeline|Timeline Play)
    (:Update
      (Transformation|SetWorldLocation (Variables|Default|Getrubber_duck_pool) (Math|Vector|MakeVector (.x _returnvalue) (.y _returnvalue) (Math|Float|Lerp (+ (Variables|Default|Getstarting%20Z) 6.0) (- (Variables|Default|Getstarting%20Z) 6.0) _newtrack_0)) false false))
    (:Finished
      (Timeline|Timeline PlayFromStart))))

(fn ConstructionScript)