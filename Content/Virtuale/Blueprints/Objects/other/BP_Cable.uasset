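; BP_Cable is a construction-script actor that builds a cable along its spline.
; For each index in a loop that runs past the last spline point, it adds a collision-free spline mesh component bent between that point and the next along the Z forward axis.
; Each component gets its own dynamic instance of the orange grid object material, and the parent construction script is called inside the loop.
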(fn ConstructionScript
  (bind _spline (Variables|Default|GetSpline))
  (for _index (range 0 (+ (Spline|GetNumberOfSplinePoints (Variables|Default|GetSpline)) 2))
    (bind _returnvalue (AddComponent|AddSplineMeshComponent false))
    (Collision|SetCollisionEnabled _returnvalue "NoCollision")
    (bind _returnvalue_2 (Rendering|Material|CreateDynamicMaterialInstance "/Game/Virtuale/Shaders/Grids_and_Wires/M_Grid_Object_orange.M_Grid_Object_orange" "None" "None" :!class /Script/Engine.KismetMaterialLibrary))
    (Rendering|Material|SetMaterial _returnvalue 0 _returnvalue_2)
    (SplineMesh|SetForwardAxis _returnvalue "Z" true)
    (SplineMesh|SetStartandEnd _returnvalue (.Location (Spline|GetLocationandTangentatSplinePoint _spline _index "Local")) (.Tangent (Spline|GetLocationandTangentatSplinePoint _spline _index "Local")) (.Location (Spline|GetLocationandTangentatSplinePoint _spline (+ _index 1) "Local")) (.Tangent (Spline|GetLocationandTangentatSplinePoint _spline (+ _index 1) "Local")) true :!class /Script/Engine.SplineMeshComponent)
    (|CallParentFunction)))