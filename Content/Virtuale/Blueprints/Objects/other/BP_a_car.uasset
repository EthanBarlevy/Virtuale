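; BP_a_car is a car prop that picks a random paint scheme for its sports car meshes.
; The construction script rolls a random index below four and uses it to set the first material on both the SportsCar and SportsCarWire meshes from two parallel material arrays, so body and wire variants stay paired.
; BeginPlay is empty, so the color is chosen only at construction.
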(event EventBeginPlay)

(fn ConstructionScript
  (Variables|Default|SetNewVar_1 (Math|Random|RandomInteger 4))
  (Rendering|Material|SetMaterial (Variables|Default|GetSportsCar) 0 (Utilities|Array|Get(acopy) (Variables|Default|GetNewVar) (Variables|Default|GetNewVar_1)))
  (Rendering|Material|SetMaterial (Variables|Default|GetSportsCar_Wire) 0 (Utilities|Array|Get(acopy) (Variables|Default|GetNewVar_0) (Variables|Default|GetNewVar_1))))