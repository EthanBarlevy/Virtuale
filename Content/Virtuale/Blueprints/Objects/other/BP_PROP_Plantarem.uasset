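; BP_PROP_Plantarem is an animated planetarium prop with a sun, several planets and four spinning pole components.
; Every Tick adds local rotation to each part, driven by four shared Rotation variables.
; The poles yaw by negated rates, one variable each, while the sun pitches and the planets yaw or roll.
; Steps are not scaled by delta time, so spin speed depends on frame rate.
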(event EventTick
  (params (DeltaSeconds :type Float%20%28single-precision%29))
  (bind _rotation_1 (Variables|Default|GetRotation%201))
  (bind _rotation_4 (Variables|Default|GetRotation%204))
  (Transformation|AddLocalRotation (Variables|Default|GetSUN) (Math|Rotator|MakeRotator 0.0 _rotation_1 0.0) false false)
  (Transformation|AddLocalRotation (Variables|Default|GetSpinny%20Poll%201) (Math|Rotator|MakeRotator 0.0 0.0 (* -1.0 _rotation_1)) false false)
  (Transformation|AddLocalRotation (Variables|Default|GetPlanet_1) (Math|Rotator|MakeRotator 0.0 0.0 _rotation_4) false false)
  (Transformation|AddLocalRotation (Variables|Default|GetSpinny%20Poll%202) (Math|Rotator|MakeRotator 0.0 0.0 (* -1.0 (Variables|Default|GetRotation%202))) false false)
  (Transformation|AddLocalRotation (Variables|Default|GetPlanet_11) (Math|Rotator|MakeRotator 0.0 0.0 _rotation_1) false false)
  (Transformation|AddLocalRotation (Variables|Default|GetSpinny%20Poll%203) (Math|Rotator|MakeRotator 0.0 0.0 (* -1.0 (Variables|Default|GetRotation%203))) false false)
  (Transformation|AddLocalRotation (Variables|Default|GetPlanet_2) (Math|Rotator|MakeRotator _rotation_1 0.0 0.0) false false)
  (Transformation|AddLocalRotation (Variables|Default|GetSpinny%20Poll%204) (Math|Rotator|MakeRotator 0.0 0.0 (* -1.0 _rotation_4)) false false)
  (Transformation|AddLocalRotation (Variables|Default|GetPlanet_7) (Math|Rotator|MakeRotator 0.0 0.0 _rotation_1) false false))

(fn ConstructionScript)