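; BP_Hacking_tablet is an interactable hacking tablet prop with an animated, flickering look.
; A looping half-second timer steps through an array of static meshes as flipbook frames, applied to both the tablet frame and its wire component.
; Each tick also shuffles a material array to randomise four named button slots on the frame.
; Enact forwards the key type to the next link in its interaction chain, then calls the parent.
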(event Custom|ChangeFrame_Event
  (bind _materalref (Variables|Default|GetMateralREF))
  (bind _materalref_2 (Variables|Default|GetMateralREF))
  (bind _materalref_3 (Variables|Default|GetMateralREF))
  (bind _materalref_4 (Variables|Default|GetMateralREF))
  (bind _tabletframe1 (Variables|Default|GetTabletFrame1))
  (Components|StaticMesh|SetStaticMesh (Variables|Default|GetTabletFrame1) (Utilities|Array|Get(acopy) (Variables|Default|GetFrames) (Variables|Default|GetFrameIDX)))
  (Components|StaticMesh|SetStaticMesh (Variables|Default|GetTabletFrame_Wire) (Utilities|Array|Get(acopy) (Variables|Default|GetFrames) (Variables|Default|GetFrameIDX)))
  ;[1 1 1] Buttons
  (Utilities|Array|Shuffle _materalref_2)
  (Rendering|Material|SetMaterialbyName _tabletframe1 "Material.006" (Utilities|Array|Get(acopy) _materalref_2 1))
  (Utilities|Array|Shuffle _materalref_3)
  (Rendering|Material|SetMaterialbyName _tabletframe1 "Material.007" (Utilities|Array|Get(acopy) _materalref_3 1))
  (Utilities|Array|Shuffle _materalref_4)
  (Rendering|Material|SetMaterialbyName _tabletframe1 "Material.008" (Utilities|Array|Get(acopy) _materalref_4 1))
  (Utilities|Array|Shuffle _materalref)
  (Rendering|Material|SetMaterialbyName _tabletframe1 "Material.009" (Utilities|Array|Get(acopy) _materalref 1))
  (bind _result (Math|Integer|IncrementInt (Variables|Default|GetFrameIDX))
    (:%20%20
      (if (>= _result (Utilities|Array|Length (Variables|Default|GetFrames)))
        (Variables|Default|SetFrameIDX 0)))))

(event EventBeginPlay
  (Utilities|Time|SetTimerbyEvent (delegate Custom|ChangeFrame_Event) 0.5 true true)
  (|CallParentFunction))

(fn ConstructionScript)

(fn Enact
  (params (KeyType :type Enum_KeyTypes%20Enum :default "NewEnumerator4"))
  (Default|NextinChain (Variables|Default|GetInteractionChain) KeyType)
  (|CallParentFunction KeyType))