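; BP_Action_StairsTeleport is an action that teleports a Puppet to a target location, by its name for moving it across stairs.
; PlayAction hides the Puppet and activates P1, moves it to TargetLocation after a short delay, then reveals it and activates P2 after another.
; The action then calls EndAction to report that it has finished.
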(event EventPlayAction
  (Rendering|SetActorHiddenInGame (Variables|Default|GetPuppet) true)
  (Components|Activation|Activate (Variables|Default|GetP1) true)
  (Utilities|FlowControl|Delay 0.5)
  (Transformation|SetActorLocation (Variables|Default|GetPuppet) (Variables|Default|GetTarget%20Location) false false)
  (Utilities|FlowControl|Delay 0.5)
  (Rendering|SetActorHiddenInGame (Variables|Default|GetPuppet) false)
  (Components|Activation|Activate (Variables|Default|GetP2) true)
  (CallFunction|EndAction true))

(fn ConstructionScript
  (|CallParentFunction))