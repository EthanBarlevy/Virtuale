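; BP_PropBase is a base prop that can switch between opaque and see-through states.
; MakeTransparent hides opaque meshes, shows translucent ones and makes the former ignore a custom trace channel; MakeOpaque reverses this, through gates opened on BeginPlay.
; Above a height threshold, the construction script collects every static mesh as opaque, then calls its parent.
; It clears the translucent list, and the node that would refill it is disconnected.
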(event Custom|MakeTransparent
  (Utilities|FlowControl|Gate true
    (:Exit
      (for _array_element (Variables|Default|GetOpaqueMeshes_0)
        (Rendering|SetVisibility _array_element false false)
        (Collision|SetCollisionResponsetoChannel _array_element "ECC_GameTraceChannel1" "ECR_Ignore")
        (for _array_element_2 (Variables|Default|GetTranslucentMeshes_0)
          (Rendering|SetVisibility _array_element_2 true false))))))

(event Custom|MakeOpaque
  (Utilities|FlowControl|Gate true
    (:Exit
      (for _array_element (Variables|Default|GetOpaqueMeshes_0)
        (Rendering|SetVisibility _array_element true false)
        (Collision|SetCollisionResponsetoChannel _array_element "ECC_GameTraceChannel1" "ECR_Block")
        (for _array_element_2 (Variables|Default|GetTranslucentMeshes_0)
          (Rendering|SetVisibility _array_element_2 false false))))))

(event EventBeginPlay
  (Utilities|FlowControl|Sequence
    (:then_0
      (Utilities|FlowControl|Gate true) ; enters at Open
    )
    (:then_1
      (Utilities|FlowControl|Gate true) ; enters at Open
    )))

(fn ConstructionScript
  (if (> (.z (.location (Transformation|GetWorldTransform (Variables|Default|GetDefaultSceneRoot)))) 249.0)
    (Utilities|Array|Clear (Variables|Default|GetOpaqueMeshes_0))
    (Utilities|Array|Clear (Variables|Default|GetTranslucentMeshes_0))
    (for _array_element (Actor|GetComponentsByClass "/Script/Engine.StaticMeshComponent")
      (Utilities|Array|Add (Variables|Default|GetOpaqueMeshes_0) _array_element))
    (|CallParentFunction)))