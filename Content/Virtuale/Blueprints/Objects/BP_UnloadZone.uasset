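; BP_UnloadZone is an object that converts a unit's carried loot into money.
; On BeginPlay it binds a handler to the grid manager's OnUnitEnterTileSimulate event.
; The handler casts the unit to BP_Unit_Stats_Anim, adds each loot value to the BP_GI_ATBTT game instance's money, then clears the loot.
; The handler does not check the grid index, so the graph itself does not restrict unloading to a particular tile.
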(event Custom|Empty
  (params (Unit :type BP%20Unit%20Object%20Reference) (GridIndex :type Integer))
  (bind _asbp_unit_stats_anim (Utilities|Casting|CastToBP_Unit_Stats_Anim Unit))
  (for _array_element (Variables|/Game/AdvancedTurnBasedTileToolkit/Maps/Experimental/StatSystem/Units/BP_Unit_Stats_Anim.BP_Unit_Stats_Anim_C|GetLoot _asbp_unit_stats_anim)
    (bind _asbp_gi_atbtt (Utilities|Casting|CastToBP_GI_ATBTT (Game|GetGameInstance)))
    (Default|AddMoney _asbp_gi_atbtt (.Value (Utilities|Struct|BreakST_Loot _array_element))))
  (Utilities|Array|Clear (Variables|/Game/AdvancedTurnBasedTileToolkit/Maps/Experimental/StatSystem/Units/BP_Unit_Stats_Anim.BP_Unit_Stats_Anim_C|GetLoot _asbp_unit_stats_anim)))

(event EventBeginPlay
  (EventDispatchers|BindEventtoOnUnitEnterTileSimulate (Variables|Default|GetGridManagerRef) (delegate Custom|Empty)))

(fn ConstructionScript)