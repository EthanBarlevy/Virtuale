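; BP_FirePlace is a fireplace object that fakes flickering flames by randomly spinning its fire pieces.
; On BeginPlay it starts a looping half-second timer that calls FireAnimation, then runs the parent BeginPlay.
; Each tick of the timer gives the three BonfireFire components a new random world yaw, with pitch and roll held at zero.
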(event Custom|Fire%20Animation
  (Transformation|SetWorldRotation (Variables|Default|GetBonfire_Fire1) (Math|Rotator|MakeRotator 0.0 0.0 (Math|Random|RandomFloatinRange 0.0 3.6e+02)) false false)
  (Transformation|SetWorldRotation (Variables|Default|GetBonfire_Fire2) (Math|Rotator|MakeRotator 0.0 0.0 (Math|Random|RandomFloatinRange 0.0 3.6e+02)) false false)
  (Transformation|SetWorldRotation (Variables|Default|GetBonfire_Fire) (Math|Rotator|MakeRotator 0.0 0.0 (Math|Random|RandomFloatinRange 0.0 3.6e+02)) false false))

(event EventBeginPlay
  (Utilities|Time|SetTimerbyEvent (delegate Custom|Fire%20Animation) 0.5 true)
  (|CallParentFunction))

(fn ConstructionScript)