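; Game instance that holds session-wide state for a turn-based job game: stat tables, earned money and music volume.
; Init caches stat rows and status classes, binding police arrests to halve earnings.
; Once StartGame runs and money exists, a one-second timer tests unit proximity to a hardcoded exit point, using DoOnce gates to signal job endable or not.
; It also joins selected multiplayer sessions and broadcasts music volume changes.
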(event Custom|JoinSelectedServer
  (params (SearchResult :type Blueprint%20Session%20Result%20Structure%20%28by%20ref%29))
  (|JoinSession (Game|GetPlayerController 0) SearchResult))

(event Custom|StartGame
  (Utilities|Time|SetTimerbyEvent (delegate Custom|CheckLeaving) 1.0 true))

(event Custom|CheckLeaving
  (if (> (Variables|Default|GetTotalMoneyEarned) 0.0)
    (bind _outactors (Actor|GetAllActorsOfClass "/Game/AdvancedTurnBasedTileToolkit/Maps/Experimental/StatSystem/Units/BP_Unit_Stats_Anim.BP_Unit_Stats_Anim_C"))
    (for _array_element _outactors
      (bind _gridindex (Default|GetGridIndex _array_element))
      (Variables|Default|SetReadyToLeave (< (Math|Vector|VectorLength (- (.Value (Utilities|Map|Find (Variables|/Game/AdvancedTurnBasedTileToolkit/Core/Grid/BP_GridManager.BP_GridManager_C|GetGridLocations (.GridManager (CallFunction|GetGridManager))) _gridindex)) "7602.500000,9481.873255,0.000000")) 2.5e+02)))
    (if (Variables|Default|GetReadyToLeave)
      ;[0.9699 0 1] Have a leave level ui thing
      (Utilities|FlowControl|DoOnce false :!label _label
        (:Completed
          (Default|CallJobEndable)
          (goto _label_2 Reset)))
      (else
        (Utilities|FlowControl|DoOnce false :!label _label_2
          (:Completed
            (Default|CallJobNotEndable)
            (goto _label Reset)))))))

(event Custom|Subtract%20Bail
  (Variables|Default|SetGrossGain (Variables|Default|GetTotalMoneyEarned))
  (Variables|Default|SetBailAmt (/ (Variables|Default|GetTotalMoneyEarned) 2.0))
  (Variables|Default|SetTotalMoneyEarned (- (Variables|Default|GetTotalMoneyEarned) (/ (Variables|Default|GetTotalMoneyEarned) 2.0))))

(event EventInit
  (for _array_element (Variables|Default|GetStatTables)
    (bind _outrownames (DataTable|GetDataTableRowNames _array_element))
    (for _array_element_2 _outrownames
      (bind _returnvalue (Utilities|GetDataTableRow _array_element _array_element_2)
        (:then
          (Utilities|Map|Add (Variables|Default|GetStatData) (.Stat (Utilities|Struct|BreakFStat _returnvalue)) _returnvalue)
          (if (Utilities|IsValidClass (.Status (Utilities|Struct|BreakFStat _returnvalue)))
            (Utilities|Map|Add (Variables|Default|GetStatStatuses) (.Stat (Utilities|Struct|BreakFStat _returnvalue)) (.Status (Utilities|Struct|BreakFStat _returnvalue)))
            (EventDispatchers|BindEventtoARREST (.PoliceSystem (CallFunction|GetPoliceSystem)) (delegate Custom|Subtract%20Bail))))))))

(fn AddMoney
  (params (Value :type Float%20%28double-precision%29))
  (bind _output_get (Variables|Default|SetTotalMoneyEarned (+ Value (Variables|Default|GetTotalMoneyEarned))))
  (Development|PrintString (Utilities|String|Append "$" (Utilities|String|ToString(Float) _output_get)) true true "(R=0.890826,G=0.000000,B=1.000000,A=1.000000)" 3e+01))

(fn ChangeMusicVolume
  (params (Volume :type Float%20%28double-precision%29))
  (Variables|Default|SetMusicVolume Volume)
  (Default|CallMusicChange))

(fn GetStatDatafromInstance
  (return (Variables|Default|GetStatStatuses) (Variables|Default|GetStatData)))