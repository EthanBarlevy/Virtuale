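; Turn manager for the Hydra map in the 2D turn-based tile toolkit, defining when and how the match ends.
; EndGameIfConditionMet sets GameOver and spawns a "GAME OVER" action when the grid's units form a single faction.
; With mixed factions, an already-set GameOver flag spawns "VICTORY" instead.
; Either ending switches every player controller to the idle ability, updates the game state's turn state and returns true.
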(event EventBeginPlay
  (|CallParentFunction) ; This node is disabled and will not be called.\nDrag off pins to build functionality.
)

(event Collision|EventActorBeginOverlap
  (params (OtherActor :type Actor%20Object%20Reference)))

(event EventTick
  (params (DeltaSeconds :type Float%20%28single-precision%29)))

(fn ConstructionScript
  (|CallParentFunction))

(fn EndGameifConditionMet
  (bind _values (Utilities|Map|Values (Variables|/Game/AdvancedTurnBasedTileToolkit/Core/Grid/BP_GridManager.BP_GridManager_C|GetGridUnits (.GridManager (CallFunction|GetGridManager)))))
  (bind _bcontainssinglefaction (CallFunction|CheckifContainsSingleFaction _values))
  (if _bcontainssinglefaction
    (bind _output_get (Variables|Default|SetbGameOver true))
    (if _output_get
      (Game|SpawnActorfromClass "/Game/AdvancedTurnBasedTileToolkit/Core/Actions/BP_Action_GameOver.BP_Action_GameOver_C" (Math|Transform|MakeTransform "0, 0, 0" "0, 0, 0" "1.000000,1.000000,1.000000") "AlwaysSpawn" 0 "GAME OVER" -1.0 "NewEnumerator0" 0)
      (else
        (return false)))
    (elif (Variables|Default|GetbGameOver)
      (Game|SpawnActorfromClass "/Game/AdvancedTurnBasedTileToolkit/Core/Actions/BP_Action_GameOver.BP_Action_GameOver_C" (Math|Transform|MakeTransform "0, 0, 0" "0, 0, 0" "1.000000,1.000000,1.000000") "AlwaysSpawn" 0 "VICTORY" -1.0 "NewEnumerator0" 0)
      (else
        (return false))))
  (bind _outactors (Actor|GetAllActorsOfClass "/Script/Engine.PlayerController"))
  (for _array_element _outactors
    (Class|BPIPC|ActivateAbility(Message) _array_element "/Game/AdvancedTurnBasedTileToolkit/Core/Abilities/BP_AbilityBase_Idle.BP_AbilityBase_Idle_C"))
  (Class|BPIGameState|SetTurnState(Message) (Game|GetGameState) "NewEnumerator7")
  (return (Variables|Default|GetbGameOver)))