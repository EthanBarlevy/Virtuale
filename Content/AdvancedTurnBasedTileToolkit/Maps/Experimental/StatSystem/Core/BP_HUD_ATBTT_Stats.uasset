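; HUD for the experimental stat system in the Advanced Turn Based Tile Toolkit, showing unit information on screen.
; On BeginPlay it creates the stats layout widget, adds it to the viewport and caches its nested unit stats widget.
; Its events and function act as pass-throughs to that widget, updating the display from unit data, abilities or current and max stats, and setting its visibility.
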(event EventSetUnitDisplayVisibility
  (params (Visibility :type ESlateVisibility%20Enum :default "Visible"))
  (Default|SetUnitDisplayVisibility (Variables|Default|GetUnitStatsWidget) Visibility))

(event EventUpdateUnitDisplayfromAbilities
  (params (Abilities :type Array%20of%20BP%20Ability%20Class%20References))
  (Default|UpdateUnitDisplayfromAbilities (Variables|Default|GetUnitStatsWidget) Abilities))

(event EventUpdateUnitDisplayfromUnitData
  (params (UnitData :type F%20Unit%20Structure%20%28by%20ref%29))
  (Default|UpdateUnitDisplayfromUnitData (Variables|Default|GetUnitStatsWidget) UnitData))

(event EventBeginPlay
  (bind _returnvalue (UserInterface|CreateWidget "/Game/AdvancedTurnBasedTileToolkit/Maps/Experimental/StatSystem/UI/WBP_StatsLayout.WBP_StatsLayout_C"))
  (UserInterface|Viewport|AddtoViewport _returnvalue 0)
  (Variables|Default|SetUnitStatsWidget (Variables|/Game/AdvancedTurnBasedTileToolkit/Maps/Experimental/StatSystem/UI/WBP_StatsLayout.WBP_StatsLayout_C|GetWBP_UnitStats _returnvalue)))

(fn ConstructionScript
  (|CallParentFunction))

(fn UpdateUnitDisplayfromStats
  (params (Stats :type Map%20of%20Gameplay%20Tag%20Structures%20to%20Reals) (MaxStats :type Map%20of%20Gameplay%20Tag%20Structures%20to%20Reals))
  (bind _bsuccess (Default|UpdateUnitDisplayfromStats (Variables|Default|GetUnitStatsWidget) Stats MaxStats))
  (return _bsuccess))