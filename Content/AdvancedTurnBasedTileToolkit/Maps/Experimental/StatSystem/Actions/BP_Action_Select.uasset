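; BP_Action_Select is an action in the experimental stat system of the turn-based tile toolkit that marks selection through custom depth stencil values.
; When played, it writes its Depth value as the stencil value on the Puppet, Weapon and Prop, then immediately ends the action, passing true.
; It does not toggle custom depth rendering itself, and its construction script only calls the parent.
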(event EventPlayAction
  (Rendering|SetCustomDepthStencilValue (Variables|Default|GetPuppet) (Variables|Default|GetDepth))
  (Rendering|SetCustomDepthStencilValue (Variables|Default|GetWeapon) (Variables|Default|GetDepth))
  (Rendering|SetCustomDepthStencilValue (Variables|Default|GetProp) (Variables|Default|GetDepth))
  (CallFunction|EndAction true))

(fn ConstructionScript
  (|CallParentFunction))