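; Health status for the tile toolkit's stat system that turns health loss into puppet feedback and handles unit death.
; On a decrease it spawns a Hurt animation action if health stays above zero, otherwise a red damage splash when the puppet displays Health, then calls the parent logic.
; Removing the status spawns a kill-puppet action and sends the owner a kill message, with visuals queried by message and run as spawned action actors.
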(fn RemoveStatus
  (params (OldValue :type Float%20%28double-precision%29))
  (bind _puppet (Class|BPIInitiative|GetPuppet(Message) (Components|GetOwner)))
  (Game|SpawnActorfromClass "/Game/AdvancedTurnBasedTileToolkit/Maps/Experimental/StatSystem/Actions/BP_Action_KillPuppet.BP_Action_KillPuppet_C" (Math|Transform|MakeTransform "0, 0, 0" "0, 0, 0" "1.000000,1.000000,1.000000") "AlwaysSpawn" 0 _puppet "0.000000,0.000000,0.000000" -1.0 "NewEnumerator0" 0)
  (Class|BPIUnit|KillUnit(Message) (Components|GetOwner))
  (return))

(fn RunonStatusModified
  (params (NewValue :type Float%20%28double-precision%29) (OldValue :type Float%20%28double-precision%29))
  (if (< (- NewValue OldValue) 0.0)
    (if (> NewValue 0.0)
      (bind _puppet (Class|BPIInitiative|GetPuppet(Message) (Components|GetOwner)))
      (Game|SpawnActorfromClass "/Game/AdvancedTurnBasedTileToolkit/Core/Actions/BP_Action_AnimatePuppet.BP_Action_AnimatePuppet_C" (Math|Transform|MakeTransform "0, 0, 0" "0, 0, 0" "1.000000,1.000000,1.000000") "Undefined" 0 _puppet "(TagName=\"Anim.Hurt\")" false -1.0 "NewEnumerator0" 0)
      (else
        (bind _puppet_2 (Class|BPIInitiative|GetPuppet(Message) (Components|GetOwner)))
        (if (GameplayTags|HasTag (Variables|/Game/AdvancedTurnBasedTileToolkit/Maps/Experimental/StatSystem/Core/BP_StatSplashComponent.BP_StatSplashComponent_C|GetStatsToShow (Actor|GetComponentbyClass _puppet_2 "/Game/AdvancedTurnBasedTileToolkit/Maps/Experimental/StatSystem/Core/BP_StatSplashComponent.BP_StatSplashComponent_C")) "(TagName=\"Stat.Health\")" true)
          (Game|SpawnActorfromClass "/Game/AdvancedTurnBasedTileToolkit/Maps/Experimental/StatSystem/Actions/BP_Action_SplashTextOnComponent.BP_Action_SplashTextOnComponent_C" (Math|Transform|MakeTransform "0, 0, 0" "0, 0, 0" "1.000000,1.000000,1.000000") "AlwaysSpawn" 0 (Utilities|Text|ToText(Float) (- OldValue NewValue) "HalfToEven") "(R=1.000000,G=0.000000,B=0.000000,A=1.000000)" (Actor|GetComponentbyClass _puppet_2 "/Game/AdvancedTurnBasedTileToolkit/Maps/Experimental/StatSystem/Core/BP_StatSplashComponent.BP_StatSplashComponent_C") -1.0 "NewEnumerator0" 0))))
    (|CallParentFunction NewValue OldValue)
    (return)
    (else
      (|CallParentFunction NewValue OldValue)
      (return))))