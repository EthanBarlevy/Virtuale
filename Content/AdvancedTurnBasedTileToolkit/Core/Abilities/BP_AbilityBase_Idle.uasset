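; Idle base ability for the turn-based tile toolkit that lets a player select their own units by clicking them.
; On a released primary click over a valid tile, the server looks up the unit at that index in the grid manager.
; If the ability's owner is the active player and also owns that unit, it sends the unit a select message.
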(event EventServerInteract
  (params (bValidTile :type Boolean) (ClickedIndex :type Integer) (Location :type Vector :default "0, 0, 0") (Key :type Key%20Structure :default "None") (bReleased :type Boolean) (ClickType :type EClickType%20Enum :default "NewEnumerator0") (CallingPc :type BP%20Player%20Controller%20ATBTT%20Object%20Reference))
  (bind _returnvalue (Components|GetOwner))
  (bind _gridmanagerref (Variables|Default|GetGridManagerRef))
  (bind _gridunits (Variables|/Game/AdvancedTurnBasedTileToolkit/Core/Grid/BP_GridManager.BP_GridManager_C|GetGridUnits _gridmanagerref))
  (bind (_value _returnvalue_2) (Utilities|Map|Find _gridunits ClickedIndex))
  (if bValidTile
    (if bReleased
      (switch Utilities|FlowControl|Switch|SwitchonEClickType ClickType
        (:NewEnumerator0
          (if _returnvalue_2
            (if (and (== (Variables|/Game/AdvancedTurnBasedTileToolkit/Core/BP_TurnManager.BP_TurnManager_C|GetActivePlayer (.TurnManager (CallFunction|GetTurnManager))) _returnvalue) (== _returnvalue (Components|GetOwner _value)))
              (Class|BPIInitiative|SelectActor(Message) (.Value (Utilities|Map|Find (Variables|/Game/AdvancedTurnBasedTileToolkit/Core/Grid/BP_GridManager.BP_GridManager_C|GetGridUnits (Variables|Default|GetGridManagerRef)) (Variables|Default|GetClickedIndex)))))))))))

(fn ConstructionScript
  (|CallParentFunction))