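; BP_Action_PlaySound is an action in the Advanced Turn Based Tile Toolkit that plays a sound at a world location.
; On PlayAction it passes its sound, location, volume, pitch, start time, attenuation and concurrency variables to PlaySoundAtLocation.
; It then calls EndAction immediately, so the action does not wait for the sound to finish.
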(event EventPlayAction
  (Audio|PlaySoundatLocation (Variables|Default|GetSound) (Variables|Default|GetLocation) "0, 0, 0" (Variables|Default|GetVolumeMultiplier) (Variables|Default|GetPitchMultiplier) (Variables|Default|GetStartTime) (Variables|Default|GetAttenuationSettings) (Variables|Default|GetConcurrencySettings) 0 0)
  (CallFunction|EndAction true))

(fn ConstructionScript
  (|CallParentFunction))